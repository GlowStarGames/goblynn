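; BP_Collectible is a pickup actor for Health, Mac Guffin or Currency items, collected by overlap.
; The construction script looks up mesh and idle VFX from maps keyed by collectible type.
; Overlapping a BPI_Interact implementer caches it and updates its interactable state via interface messages.
; It then plays a type-specific sound, swaps to pickup VFX, reports the type to that actor and destroys itself after a short delay.
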(event `self.ReceiveActorBeginOverlap`
  (params (OtherActor :type "Actor Object Reference"))
  (`|ExecutionSequence`
    (:`then_0`
      ;[1 1 1] Check if Overlapping Self
      (if (!= OtherActor self)
        ;[1 1 1] Check if Interactable
        (if (`KismetSystemLibrary.DoesImplementInterface` OtherActor "/Game/Game/Blueprints/Interactable/BPI_Interact.BPI_Interact_C")
          ;[1 1 1] Check if Valid
          (`/Engine/EditorBlueprintResources/StandardMacros.IsValid` (`self.Interactable`)
            (:`Is Valid`
              ;[1 1 1] Set Interactable State to Overlapping Component
              (message `/Game/Game/Blueprints/Interactable/BPI_Interact.SetInteractableState` (`self.Interactable`) false)
              (set `self.Interactable` null))
            (:`Is Not Valid`
              _))
          (set `self.Interactable` OtherActor)
          ;[1 1 1] Set to Interactable
          (message `/Game/Game/Blueprints/Interactable/BPI_Interact.SetInteractableState` (`self.Interactable`) true))))
    (:`then_1`
      ;[1 1 1] Check if Interactable
      (if (`KismetSystemLibrary.DoesImplementInterface` OtherActor "/Game/Game/Blueprints/Interactable/BPI_Interact.BPI_Interact_C")
        ;[1 1 1] Pick Up Item
        (switch `/Game/Game/Blueprints/Interactable/Enum_Collectible` (`self.Collectible`)
          (:`NewEnumerator1`
            (`GameplayStatics.PlaySoundAtLocation` "/Game/Interface_And_Item_Sounds/Cues/Futuristic_Click_02_Cue.Futuristic_Click_02_Cue" (`self.K2_GetActorLocation`) (struct) 0.3 1.0 0.0 null null null null))
          (:`NewEnumerator2`
            (`GameplayStatics.PlaySoundAtLocation` "/Game/Interface_And_Item_Sounds/Cues/Coins_15_Cue.Coins_15_Cue" (`self.K2_GetActorLocation`) (struct) 0.3 1.0 0.0 null null null null))
          (:`NewEnumerator3`
            (`GameplayStatics.PlaySoundAtLocation` "/Game/Interface_And_Item_Sounds/Cues/Coins_11_Cue.Coins_11_Cue" (`self.K2_GetActorLocation`) (struct) 0.3 1.0 0.0 null null null null)))
        (`NiagaraComponent.SetAsset` (`self.ComponentVFX`) (`BlueprintMapLibrary.Map_Find` (`self.PickupMapVFX`) (`self.Collectible`)) true)
        (message `/Game/Game/Blueprints/Interactable/BPI_Interact.ItemPickup` (`self.Interactable`) (`self.Collectible`))
        (`KismetSystemLibrary.Delay` 0.2)
        (`self.K2_DestroyActor`)))))

(fn `ItemPickup`
  (params (CollectibleType :type "/Game/Game/Blueprints/Interactable/Enum_Collectible Enum" :default "NewEnumerator0")))

(fn `UserConstructionScript`
  ;[1 1 1] Construct VXF for Collectibles
  (`NiagaraComponent.SetAsset` (`self.ComponentVFX`) (`BlueprintMapLibrary.Map_Find` (`self.AssetMapVFX`) (`self.Collectible`)) true)
  (`StaticMeshComponent.SetStaticMesh` (`self.CollectibleMesh`) (`BlueprintMapLibrary.Map_Find` (`self.MeshMap`) (`self.Collectible`))))