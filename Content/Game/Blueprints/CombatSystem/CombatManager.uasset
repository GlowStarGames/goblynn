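; CombatManager limits how many attackers can attack a single target at once.
; On BeginPlay it reads the maximum attacker count from AttackTarget through an interface message.
; HandleAttackRequest ignores the target itself, then either adds the requester to Attackers and messages it to attack, or adds it to WaitingAttackers and messages it to wait.
; Nothing here removes attackers or promotes waiting ones.
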(event `self.ReceiveBeginPlay`
  ;[1 1 1] Set Max Attackers Count
  (bind _maxattackerscount (message `/Game/Game/Blueprints/CombatSystem/BPI_AttackTarget.GetMaxAttackersCount` (`self.AttackTarget`)))
  (set `self.Max Attackers Count` _maxattackerscount))

(fn `GetMaxAttackersCount`
  (returns (MaxAttackersCount :type Integer))
  (return 0))

(fn `GetPatrolRoute`
  (returns (PatrolRoute :type "/Game/Game/Blueprints/Character/Enemy/BP_PatrolRoute Object Reference"))
  (return null))

(fn `HandleAttackRequest`
  (params (Attacker :type "Actor Object Reference"))
  (locals (NewLocalVar :type "Array of Actor Object Reference"))
  (bind _attacktarget (`self.AttackTarget`))
  ;[1 1 1] Ensure Attacker is not Attack Target
  (if (!= Attacker (`self.AttackTarget`))
    ;[1 1 1] Compare Attackers to Max Attackers Count
    (if (< (`KismetArrayLibrary.Array_Length` (`self.Attackers`)) (`self.Max Attackers Count`))
      ;[1 1 1] Add Attacker to Array
      (`KismetArrayLibrary.Array_AddUnique` (`self.Attackers`) Attacker)
      ;[1 1 1] Attack or Wait
      (message `/Game/Game/Blueprints/CombatSystem/BPI_Attacker.Attack` Attacker _attacktarget)
      (else
        (`KismetArrayLibrary.Array_AddUnique` (`self.WaitingAttackers`) Attacker)
        (message `/Game/Game/Blueprints/CombatSystem/BPI_Attacker.Wait` Attacker _attacktarget)))))

(fn `UserConstructionScript`)