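; Quest-gated door trigger that seals a quest adventurer in until the quest is complete.
; Leaving the collision box with the quest unfinished spawns BP_Door with effects and, once only, sets the quest message and shows a locked-in widget.
; Re-entering asks the QuestManager for completion, then either destroys the door with a burst or plays hit effects and a still-locked widget, removed shortly after walking away.
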(event `self.ReceiveBeginPlay`
  ;[1 1 1] Create Quest Manager Reference
  (bind _returnvalue (`GameplayStatics.GetActorOfClass` "/Game/Game/Blueprints/Quests/QuestManager.QuestManager_C"))
  (set `self.QuestManagerREF` _returnvalue))

(event `self.CollisionBox.OnComponentEndOverlap`
  (params (OverlappedComponent :type "PrimitiveComponent Object Reference") (OtherActor :type "Actor Object Reference") (OtherComp :type "PrimitiveComponent Object Reference") (OtherBodyIndex :type Integer))
  (bind (_returnvalue_x _returnvalue_y _returnvalue_z) (`KismetMathLibrary.BreakVector` (`self.K2_GetActorLocation` OtherActor)))
  (bind _wbp_wards (`self.WBP_Wards`))
  (bind (_door_location_x _door_location_y) (`KismetMathLibrary.BreakVector` (`self.Door Location`)))
  ;[1 1 1] Create Door
  (if (`KismetSystemLibrary.DoesImplementInterface` OtherActor "/Game/Game/Blueprints/Quests/BPI_Quest.BPI_Quest_C")
    (bind _bquestcomplete_ (`/Game/Game/Blueprints/Quests/BPI_Quest.CheckQuestCompletion` (`self.QuestManagerREF`) OtherActor "NewEnumerator1"))
    (if (not _bquestcomplete_)
      (`/Engine/EditorBlueprintResources/StandardMacros.IsValid` (`self.DoorREF`)
        (:`Is Valid`
          ;[1 1 1] Remove "Still Locked" Widget when walking away
          (`/Engine/EditorBlueprintResources/StandardMacros.IsValid` _wbp_wards
            (:`Is Valid`
              (`KismetSystemLibrary.Delay` 1.0)
              (`/Engine/EditorBlueprintResources/StandardMacros.IsValid` _wbp_wards
                (:`Is Valid`
                  (`WidgetBlueprintLibrary.SetInputMode_GameOnly` (`GameplayStatics.GetPlayerController` 0))
                  (`Widget.RemoveFromParent` (`self.WBP_Wards`)))))))
        (:`Is Not Valid`
          (bind _returnvalue (`|SpawnActorFromClass` "/Game/Game/Blueprints/Quests/BP_Door.BP_Door_C" (`KismetMathLibrary.MakeTransform` (`self.Door Location`) (struct) (`self.GetActorScale3D`)) "Undefined" "MultiplyWithRoot" null null))
          (set `self.DoorREF` _returnvalue)
          (`|SpawnActorFromClass` "/Game/ImproveFights_Vfx/Blueprints/BP_Explosion.BP_Explosion_C" (`KismetMathLibrary.MakeTransform` (`KismetMathLibrary.MakeVector` _returnvalue_x _door_location_y _returnvalue_z)) "Undefined" "MultiplyWithRoot" null 0.5 1.0 "/Game/ImproveFights_Vfx/Particles/P_Darkness_Hit_02.P_Darkness_Hit_02" null)
          (`GameplayStatics.PlaySoundAtLocation` "/Game/Interface_And_Item_Sounds/Cues/Gong_01_Cue.Gong_01_Cue" (`self.Door Location`) (struct) 1.0 1.0 0.0 null null null null)
          ;[1 1 1] Set Quest Requirements
          (`/Engine/EditorBlueprintResources/StandardMacros.DoOnce` false
            (:`Completed`
              (message `/Game/Game/Blueprints/Quests/BPI_Quest.SetQuest` (`self.QuestManagerREF`) "NewEnumerator1")
              ;[1 1 1] Locked In Message
              (bind _returnvalue_2 (`|CreateWidget` "/Game/Game/Widgets/WBP_LockedIn.WBP_LockedIn_C"))
              (`KismetSystemLibrary.Delay` 2.5)
              (`UserWidget.AddToViewport` _returnvalue_2 0))))))))

(event `self.CollisionBox.OnComponentBeginOverlap`
  (params (OverlappedComponent :type "PrimitiveComponent Object Reference") (OtherActor :type "Actor Object Reference") (OtherComp :type "PrimitiveComponent Object Reference") (OtherBodyIndex :type Integer) (bFromSweep :type Boolean) (SweepResult :type "HitResult Structure (by ref)"))
  (bind (_returnvalue_x _returnvalue_y _returnvalue_z) (`KismetMathLibrary.BreakVector` (`self.K2_GetActorLocation` OtherActor)))
  (bind (_door_location_x _door_location_y) (`KismetMathLibrary.BreakVector` (`self.Door Location`)))
  ;[1 1 1] Complete Quest
  ;;[1 1 1] Check for Player and Door
  (if (`KismetSystemLibrary.DoesImplementInterface` OtherActor "/Game/Game/Blueprints/Quests/BPI_Quest.BPI_Quest_C")
    (`/Engine/EditorBlueprintResources/StandardMacros.IsValid` (`self.DoorREF`)
      (:`Is Valid`
        ;;[1 1 1] Check Quest Completion
        (bind _bquestcomplete_ (`/Game/Game/Blueprints/Quests/BPI_Quest.CheckQuestCompletion` (`self.QuestManagerREF`) OtherActor "NewEnumerator1"))
        (if _bquestcomplete_
          ;;[1 1 1] Destroy Door
          (`|SpawnActorFromClass` "/Game/ImproveFights_Vfx/Blueprints/BP_Explosion.BP_Explosion_C" (`KismetMathLibrary.MakeTransform` (`self.Door Location`)) "Undefined" "MultiplyWithRoot" null 0.5 1.5 "/Niagara/DefaultAssets/Templates/Systems/RadialBurst.RadialBurst" null)
          (`GameplayStatics.PlaySoundAtLocation` "/Game/Interface_And_Item_Sounds/Cues/Special_Powerup_04_Cue.Special_Powerup_04_Cue" (`self.Door Location`) (struct) 1.0 1.0 0.0 null null null null)
          (`KismetSystemLibrary.Delay` 0.2)
          (`self.K2_DestroyActor` (`self.DoorREF`))
          (else
            ;;[1 1 1] Collide with Door
            (`KismetSystemLibrary.Delay` 0.2)
            (`|SpawnActorFromClass` "/Game/Game/Blueprints/BP_DoorHit.BP_DoorHit_C" (`KismetMathLibrary.MakeTransform` (`KismetMathLibrary.MakeVector` _returnvalue_x _door_location_y _returnvalue_z)) "Undefined" "MultiplyWithRoot" null 0.2 "/Game/ImproveFights_Vfx/Particles/P_WeaponDarkness_Hit.P_WeaponDarkness_Hit" 1.0 null)
            (`GameplayStatics.PlaySoundAtLocation` "/Game/Interface_And_Item_Sounds/Cues/Futuristic_Click_10_Cue.Futuristic_Click_10_Cue" (`KismetMathLibrary.MakeVector` _returnvalue_x _door_location_y _returnvalue_z) (struct) 1.0 1.0 0.0 null null null null)
            (`/Engine/EditorBlueprintResources/StandardMacros.IsValid` null
              (:`Is Valid`
                (`UserWidget.AddToViewport` (`self.WBP_Wards`) 0))
              (:`Is Not Valid`
                (bind _returnvalue (`|CreateWidget` "/Game/Game/Widgets/WBP_StillLocked.WBP_StillLocked_C"))
                (`UserWidget.AddToViewport` _returnvalue 0)
                (set `self.WBP_Wards` _returnvalue)))))))))

(fn `CheckActiveQuests`
  (returns (ActiveQuests :type "Array of /Game/Game/Blueprints/Quests/Enum_QuestList Enum"))
  (return))

(fn `CheckQuestCompletion`
  (params (Adventurer :type "Actor Object Reference") (Quest :type "/Game/Game/Blueprints/Quests/Enum_QuestList Enum" :default "NewEnumerator0"))
  (returns (`bQuestComplete?` :type Boolean))
  (return false))

(fn `GetCollectedItemNumber`
  (params (Collectible :type "/Game/Game/Blueprints/Interactable/Enum_Collectible Enum" :default "NewEnumerator0"))
  (returns (QuantityCollected :type Integer))
  (return 0))

(fn `TurnInQuest`
  (params (Quest :type "/Game/Game/Blueprints/Quests/Enum_QuestList Enum" :default "NewEnumerator0") (Adventurer :type "Actor Object Reference"))
  (return))

(fn `UserConstructionScript`)