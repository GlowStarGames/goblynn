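; Quest manager that tracks active quests, checks their completion and handles turn-in for an adventurer.
; SetQuest adds unique entries to the active list, and per-quest map lookups supply required items, quantities and rewards.
; CheckQuestCompletion gets the adventurer's item count through an interface message and compares it to the requirement.
; TurnInQuest sends requirement and reward data to the adventurer, removes the quest and resets the shared completion flag.
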(event `/Game/Game/Blueprints/Quests/BPI_Quest.SetQuest`
  (params (Quest :type "/Game/Game/Blueprints/Quests/Enum_QuestList Enum" :default "NewEnumerator0"))
  ;[1 1 1] Set Quest
  (`KismetArrayLibrary.Array_AddUnique` (`self.ActiveQuest`) Quest)
  (for _ (`self.ActiveQuest`)
    _))

(fn `CheckActiveQuests`
  (returns (ActiveQuests :type "Array of /Game/Game/Blueprints/Quests/Enum_QuestList Enum"))
  (return (`self.ActiveQuest`)))

(fn `CheckQuestCompletion`
  (params (Adventurer :type "Actor Object Reference") (Quest :type "/Game/Game/Blueprints/Quests/Enum_QuestList Enum" :default "NewEnumerator0"))
  (returns (`bQuestComplete?` :type Boolean))
  ;[1 1 1] Find Item Associated with Quest and Ask Adventurer for Quantity
  (bind _quantitycollected (message `/Game/Game/Blueprints/Quests/BPI_Quest.GetCollectedItemNumber` Adventurer (`BlueprintMapLibrary.Map_Find` (`self.QuestItemRequirements`) Quest)))
  ;[1 1 1] Find Quest Requirement and Compare Collected Item Quantity
  (if (>= _quantitycollected (`BlueprintMapLibrary.Map_Find` (`self.QuestQuantityRequirements`) Quest))
    ;[1 1 1] Set Quest Completion
    (set `self.bQuestComplete?` true)
    (else
      (set `self.bQuestComplete?` false)))
  (return (`self.bQuestComplete?`)))

(fn `GetCollectedItemNumber`
  (params (Collectible :type "/Game/Game/Blueprints/Interactable/Enum_Collectible Enum" :default "NewEnumerator0"))
  (returns (QuantityCollected :type Integer))
  (return 0))

(fn `TurnInQuest`
  (params (Quest :type "/Game/Game/Blueprints/Quests/Enum_QuestList Enum" :default "NewEnumerator0") (Adventurer :type "Actor Object Reference"))
  ;[1 1 1] Turn In Quest
  (message `/Game/Game/Blueprints/Quests/BPI_Quest.CollectQuest` Adventurer (`BlueprintMapLibrary.Map_Find` (`self.QuestItemRequirements`) Quest) (`BlueprintMapLibrary.Map_Find` (`self.QuestQuantityRequirements`) Quest) (`BlueprintMapLibrary.Map_Find` (`self.QuestReward`) Quest) (`BlueprintMapLibrary.Map_Find` (`self.RewardQuantity`) Quest))
  ;[1 1 1] Remove from Active Quests
  (`KismetArrayLibrary.Array_RemoveItem` (`self.ActiveQuest`) Quest)
  (set `self.bQuestComplete?` false)
  (return))

(fn `UserConstructionScript`)