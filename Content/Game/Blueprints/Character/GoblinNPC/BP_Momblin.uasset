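; BP_Momblin is an interactable goblin NPC that holds a dialogue and hands out a collectible.
; Interacting stores the instigator, asks the QuestManager whether a quest is complete to pick the QuestComplete branch, then opens dialogue.
; Closing the conversation notifies the instigator and spawns a BP_Collectible at StewSpawn on every close.
; Interactable state toggles the name and button prompts, with a pop sound on show; quest functions here are empty stubs.
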(event `self.SetInteractableState`
  (params (`bCanShowInteract?` :type Boolean))
  ;[1 1 1] Name Appear/Disappear
  (if `bCanShowInteract?`
    (`GameplayStatics.PlaySoundAtLocation` "/Game/Interface_And_Item_Sounds/Cues/Abstract_Pop_01_Cue.Abstract_Pop_01_Cue" (`self.K2_GetActorLocation`) (struct) 0.5 1.0 0.0 null null null null)
    (`SceneComponent.SetVisibility` (`self.ButtonPrompt`) true false)
    (`SceneComponent.SetVisibility` (`self.Txt_Prompt`) true false)
    (else
      (`SceneComponent.SetVisibility` (`self.ButtonPrompt`) false false)
      (`SceneComponent.SetVisibility` (`self.Txt_Prompt`) false false))))

(event `self.ConversationClosed`
  (params (Speaker :type Text))
  ;[1 1 1] Conversation Closed
  (message `/Game/Game/Blueprints/Interactable/BPI_Interact.ConversationClosed` (`self.InteractInstigator`) (`self.Name`))
  (`|SpawnActorFromClass` "/Game/Game/Blueprints/Interactable/BP_Collectible.BP_Collectible_C" (`KismetMathLibrary.MakeTransform` (`self.StewSpawn`)) "AlwaysSpawn" "MultiplyWithRoot" null null))

(event `self.Interact`
  (params (Instigator :type "Actor Object Reference"))
  (bind _ac_dialogue_momblin (`self.AC_Dialogue_Momblin`))
  ;[1 1 1] Open Dialogue on Interact
  (bind _output_get (set `self.InteractInstigator` Instigator))
  (bind _bquestcomplete_ (message `/Game/Game/Blueprints/Quests/BPI_Quest.CheckQuestCompletion` (`self.QuestManagerREF`) _output_get "NewEnumerator1"))
  (if _bquestcomplete_
    (set `/Game/Game/Blueprints/Dialogue/AC_DialogueBase.ActiveDialogueBranch` "QuestComplete" _ac_dialogue_momblin))
  (`/Game/Game/Blueprints/Dialogue/AC_DialogueBase.OpenDialogue` _ac_dialogue_momblin))

(event `self.ReceiveBeginPlay`
  ;[1 1 1] Create References
  (bind _returnvalue (`GameplayStatics.GetActorOfClass` "/Game/Game/Blueprints/Quests/QuestManager.QuestManager_C"))
  (set `self.QuestManagerREF` _returnvalue)
  (`TextRenderComponent.K2_SetText` (`self.Txt_Prompt`) (`self.Name`)))

(fn `CheckActiveQuests`
  (returns (ActiveQuests :type "Array of /Game/Game/Blueprints/Quests/Enum_QuestList Enum"))
  (return))

(fn `CheckQuestCompletion`
  (params (Adventurer :type "Actor Object Reference") (Quest :type "/Game/Game/Blueprints/Quests/Enum_QuestList Enum" :default "NewEnumerator0"))
  (returns (`bQuestComplete?` :type Boolean))
  (return false))

(fn `GetCollectedItemNumber`
  (params (Collectible :type "/Game/Game/Blueprints/Interactable/Enum_Collectible Enum" :default "NewEnumerator0"))
  (returns (QuantityCollected :type Integer))
  (return 0))

(fn `TurnInQuest`
  (params (Quest :type "/Game/Game/Blueprints/Quests/Enum_QuestList Enum" :default "NewEnumerator0") (Adventurer :type "Actor Object Reference"))
  (return))

(fn `UserConstructionScript`)