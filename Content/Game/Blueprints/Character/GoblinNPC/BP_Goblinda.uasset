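; Goblinda, a quest-giver NPC that assigns a quest, accepts its turn-in and then leaves the level.
; Interact queries the QuestManager through messages to pick the assign or completion branch before opening her dialogue component.
; Closing dialogue with TurnItIn set turns in the quest once and starts a timer that retries until the player no longer overlaps her capsule, then destroys her.
; Interactable state toggles her name and button prompt.
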(event `GoHome`
  ;[1 1 1] Send Linda Home
  (if (`PrimitiveComponent.IsOverlappingActor` (`self.CapsuleComponent`) (`self.InteractInstigator`))
    (`KismetSystemLibrary.K2_SetTimerDelegate` (delegate `GoHome`) 10.0)
    (else
      (`self.K2_DestroyActor`))))

(event `/Game/Game/Blueprints/Interactable/BPI_Interact.ConversationClosed`
  (params (Speaker :type Text))
  ;[1 1 1] Conversation Closed
  (set `self.bQuestGiven?` true)
  (message `/Game/Game/Blueprints/Interactable/BPI_Interact.ConversationClosed` (`self.InteractInstigator`) (`self.Name`))
  (if (`/Game/Game/Blueprints/Dialogue/AC_DialogueBase.bTurnItIn?` (`self.AC_Dialogue_Goblinda`))
    (`/Engine/EditorBlueprintResources/StandardMacros.DoOnce` false
      (:`Completed`
        (message `/Game/Game/Blueprints/Quests/BPI_Quest.TurnInQuest` (`self.QuestManagerREF`) (`self.Quest`) (`self.InteractInstigator`))
        (`KismetSystemLibrary.K2_SetTimerDelegate` (delegate `GoHome`) 10.0)))
    (else
      (set `/Game/Game/Blueprints/Quests/QuestManager.bQuestComplete?` false (`self.QuestManagerREF`)))))

(event `/Game/Game/Blueprints/Interactable/BPI_Interact.Interact`
  (params (Instigator :type "Actor Object Reference"))
  (bind _ac_dialogue_goblinda (`self.AC_Dialogue_Goblinda`))
  (bind _ac_dialogue_goblinda_2 (`self.AC_Dialogue_Goblinda`))
  ;[1 1 1] Check Quest Status and Open Dialogue
  (bind _output_get (set `self.InteractInstigator` Instigator))
  (bind _activequests (message `/Game/Game/Blueprints/Quests/BPI_Quest.CheckActiveQuests` (`self.QuestManagerREF`)))
  (if (`/Game/Game/Blueprints/Dialogue/AC_DialogueBase.bTurnItIn?` (`self.AC_Dialogue_Goblinda`))
    (`/Game/Game/Blueprints/Dialogue/AC_DialogueBase.OpenDialogue` _ac_dialogue_goblinda :!label _label)
    (else
      (if (>= (`KismetArrayLibrary.Array_Find` _activequests (`self.Quest`)) 0)
        (if (`self.bQuestGiven?`)
          (bind _bquestcomplete_ (message `/Game/Game/Blueprints/Quests/BPI_Quest.CheckQuestCompletion` (`self.QuestManagerREF`) _output_get (`self.Quest`)))
          (if _bquestcomplete_
            (set `/Game/Game/Blueprints/Dialogue/AC_DialogueBase.ActiveDialogueBranch` "QuestComplete" _ac_dialogue_goblinda)
            (goto _label)
            (else
              (goto _label)))
          (else
            _)))
      (message `/Game/Game/Blueprints/Quests/BPI_Quest.SetQuest` (`self.QuestManagerREF`) (`self.Quest`))
      (set `/Game/Game/Blueprints/Dialogue/AC_DialogueBase.ActiveDialogueBranch` "AssignQuest" _ac_dialogue_goblinda_2)
      (`/Game/Game/Blueprints/Dialogue/AC_DialogueBase.OpenDialogue` _ac_dialogue_goblinda_2))))

(event `self.ReceiveBeginPlay`
  ;[1 1 1] Create Quest Manager Reference
  (bind _returnvalue (`GameplayStatics.GetActorOfClass` "/Game/Game/Blueprints/Quests/QuestManager.QuestManager_C"))
  (set `self.QuestManagerREF` _returnvalue)
  (`TextRenderComponent.K2_SetText` (`self.Txt_Prompt`) (`self.Name`))
  (set `self.bQuestGiven?` false))

(event `/Game/Game/Blueprints/Interactable/BPI_Interact.SetInteractableState`
  (params (`bCanShowInteract?` :type Boolean))
  ;[1 1 1] Name Appear/Disappear
  (if `bCanShowInteract?`
    (`GameplayStatics.PlaySoundAtLocation` "/Game/Interface_And_Item_Sounds/Cues/Abstract_Pop_01_Cue.Abstract_Pop_01_Cue" (`self.K2_GetActorLocation`) (struct) 0.5 1.0 0.0 null null null null)
    (`SceneComponent.SetVisibility` (`self.ButtonPrompt`) true false)
    (`SceneComponent.SetVisibility` (`self.Txt_Prompt`) true false)
    (else
      (`SceneComponent.SetVisibility` (`self.ButtonPrompt`) false false)
      (`SceneComponent.SetVisibility` (`self.Txt_Prompt`) false false))))

(fn `CheckActiveQuests`
  (returns (ActiveQuests :type "Array of /Game/Game/Blueprints/Quests/Enum_QuestList Enum"))
  (return))

(fn `CheckQuestCompletion`
  (params (Adventurer :type "Actor Object Reference") (Quest :type "/Game/Game/Blueprints/Quests/Enum_QuestList Enum" :default "NewEnumerator0"))
  (returns (`bQuestComplete?` :type Boolean))
  (return false))

(fn `GetCollectedItemNumber`
  (params (Collectible :type "/Game/Game/Blueprints/Interactable/Enum_Collectible Enum" :default "NewEnumerator0"))
  (returns (QuantityCollected :type Integer))
  (return 0))

(fn `TurnInQuest`
  (params (Quest :type "/Game/Game/Blueprints/Quests/Enum_QuestList Enum" :default "NewEnumerator0") (Adventurer :type "Actor Object Reference"))
  (return))

(fn `UserConstructionScript`)