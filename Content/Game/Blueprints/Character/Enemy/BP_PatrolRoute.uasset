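; BP_PatrolRoute defines a spline-based patrol path for enemies, tracking the current point along it.
; IncrementPatrolRoute steps PatrolIndex by Direction, ping-ponging between the first and last spline points.
; At either end, it waits through a short delay before flipping Direction; the index itself changes before the delay.
; GetSplinePointAsWorldPosition returns the current point's world-space location.
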(event `IncrementPatrolRoute`
  ;[1 1 1] Increment Patrol Index forward or backward
  (bind _output_get (set `self.PatrolIndex` (+ (`self.PatrolIndex`) (`self.Direction`))))
  ;[1 1 1] Change Direction at the end of the Spline
  (if (== _output_get (- (`SplineComponent.GetNumberOfSplinePoints` (`self.PatrolRoute`)) 1))
    (`KismetSystemLibrary.Delay` 2.0)
    (set `self.Direction` -1)
    (else
      ;[1 1 1] Set Direction at the beginning of the Spline
      (if (== (`self.PatrolIndex`) 0)
        (`KismetSystemLibrary.Delay` 2.0)
        (set `self.Direction` 1)))))

(fn `GetSplinePointAsWorldPosition`
  (returns (Location :type "Vector Structure"))
  (return (`SplineComponent.GetLocationAtSplinePoint` (`self.PatrolRoute`) (`self.PatrolIndex`) "World")))

(fn `UserConstructionScript`)