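; Ghoul enemy character that patrols, alerts and attacks when a BP_Goblin enters its alert radius, and returns to patrol when that target leaves.
; Events drive state changes on its AIC_EnemyBase controller, playing montages and sounds for alert, hit and death.
; Punches alternate left and right montages via FlipFlop and deal damage through a forward sphere trace.
; AC_DamageSystem handles health and dispatches hit and death responses, with death spawning an explosion before destroying the actor.
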(event `self.ReceiveBeginPlay`
  ;[1 0.526 0.526] Change Enemy State
  ;;[1 1 1] Connect to AI State Controls
  (bind _asaic_enemy_base (cast `/Game/Game/Blueprints/Character/Enemy/AI/AIC_EnemyBase` (`AIBlueprintHelperLibrary.GetAIController` self)))
  (set `self.As AIC Enemy Base` _asaic_enemy_base)
  (set `self.bIsAttacking` false)
  (set `self.bIsAlerted` false)
  (set `self.bIsDead` false))

(event `self.EnemyAlertRadius.OnComponentEndOverlap`
  (params (OverlappedComponent :type "PrimitiveComponent Object Reference") (OtherActor :type "Actor Object Reference") (OtherComp :type "PrimitiveComponent Object Reference") (OtherBodyIndex :type Integer))
  ;[1 0.526 0.526] Change Enemy State
  ;;[1 1 1] Resume Patrol
  (if (and (== OtherActor (`self.AttackTarget`)) (not (`self.bIsDead`)))
    (`/Game/Game/Blueprints/Character/Enemy/AI/AIC_EnemyBase.SetStateAsPatrol` (`self.As AIC Enemy Base`))
    (set `self.bIsAlerted` false)
    (`KismetSystemLibrary.PrintString` "Set State Patrol")))

(event `/Game/Game/Blueprints/Character/Enemy/AI/BPI_EnemyAI.Alert`
  ;[1 0.526 0.526] Change Enemy State
  ;;[1 1 1] Play Alert
  (if (`self.bIsAlerted`)
    (`|PlayMontage` (`self.Mesh`) "/Game/Game/Blueprints/Animations/Montages/Montage_Ghoul_Agr.Montage_Ghoul_Agr"
      (:`then`
        (`GameplayStatics.PlaySoundAtLocation` "/Game/HumanVocalizations/HumanMaleB/Cues/voice_male_b_growl_08_Cue.voice_male_b_growl_08_Cue" (`self.K2_GetActorLocation`) (struct) 0.5 1.0 0.0 null null null null)
        (`KismetSystemLibrary.Delay` 2.5)
        (set `self.bIsAlerted` false)
        (`/Game/Game/Blueprints/Character/Enemy/AI/AIC_EnemyBase.SetStateAsAttacking` (`self.As AIC Enemy Base`) (`self.AttackTarget`))
        (`self.OnAlertEnd`)))))

(event `self.EnemyAlertRadius.OnComponentBeginOverlap`
  (params (OverlappedComponent :type "PrimitiveComponent Object Reference") (OtherActor :type "Actor Object Reference") (OtherComp :type "PrimitiveComponent Object Reference") (OtherBodyIndex :type Integer) (bFromSweep :type Boolean) (SweepResult :type "HitResult Structure (by ref)"))
  ;[1 0.526 0.526] Change Enemy State
  ;;[1 1 1] Check for Alert when Overlap Begins
  (if (`KismetMathLibrary.ClassIsChildOf` (`GameplayStatics.GetObjectClass` OtherActor) "/Game/Game/Blueprints/Character/PlayerGoblin/BP_Goblin.BP_Goblin_C")
    (if (not (`self.bIsAlerted`))
      (set `self.AttackTarget` OtherActor)
      ;;[1 1 1] Set State as Alert
      (set `self.bIsAlerted` true)
      (`/Game/Game/Blueprints/Character/Enemy/AI/AIC_EnemyBase.SetStateAsAlert` (`self.As AIC Enemy Base`) (`self.AttackTarget`)))))

(event `Punch`
  (bind _returnvalue (`self.K2_GetActorLocation`))
  (bind _mesh (`self.Mesh`))
  ;[1 0 0] Combat
  ;;[1 1 1] Punch Attack
  ;;;[1 1 1] Create Punch Loop
  (`KismetSystemLibrary.Delay` 0.2)
  (if (not (`/Game/Game/Blueprints/DamageSystem/AC_DamageSystem_New.bIsDead` (`self.AC_DamageSystem_New`)))
    ;;;[1 1 1] Set bIsAttacking
    (if (not (`self.bIsAttacking`))
      (set `self.bIsAttacking` true)
      (`|ExecutionSequence`
        (:`then_0`
          ;;;[1 1 1] Damage Radius
          (bind (_outhit _returnvalue_2) (`KismetSystemLibrary.SphereTraceSingleForObjects` :`Start` _returnvalue :`End` (+ _returnvalue (* (`self.GetActorForwardVector`) 80.0)) :`Radius` 50.0 :`ObjectTypes` (`|MakeArray` "ObjectTypeQuery3" :!type "EObjectTypeQuery Enum") :`TraceColor` (struct :`R` 1.0 :`B` 0.642941 :`A` 1.0) :`TraceHitColor` (struct :`R` 0.817354 :`G` 1.0 :`A` 1.0) :`DrawTime` 1.0))
          ;;;[1 1 1] Do Damage
          (if _returnvalue_2
            (message `/Game/Game/Blueprints/DamageSystem/BPI_Damageable.TakeDamage` (`.HitActor` (`GameplayStatics.BreakHitResult` _outhit)) (make `/Game/Game/Blueprints/DamageSystem/S_DamageInfo` 1.0 "NewEnumerator1" "NewEnumerator1"))))
        (:`then_1`
          ;;;[1 1 1] Punch Animation
          (`/Engine/EditorBlueprintResources/StandardMacros.FlipFlop`
            (:`A`
              (`|PlayMontage` _mesh "/Game/Game/Blueprints/Animations/Montages/Montage_Ghoul_AttackR.Montage_Ghoul_AttackR"
                (:`then`
                  (`KismetSystemLibrary.Delay` 0.1)
                  (`GameplayStatics.PlaySoundAtLocation` "/Game/SFX_Woosh/woosh1_Cue.woosh1_Cue" (`self.K2_GetActorLocation`) (struct) 0.5 1.0 0.0 null null null null))))
            (:`B`
              (`|PlayMontage` _mesh "/Game/Game/Blueprints/Animations/Montages/Montage_Ghoul_AttackL.Montage_Ghoul_AttackL"
                (:`then`
                  (`KismetSystemLibrary.Delay` 0.1)
                  (`GameplayStatics.PlaySoundAtLocation` "/Game/SFX_Woosh/woosh2_Cue.woosh2_Cue" (`self.K2_GetActorLocation`) (struct) 0.5 1.0 0.0 null null null null)))))
          (set `self.bIsAttacking` false)
          (`self.OnAttackEnd`))))))

(event `DamageResponse`
  (params (DamageResponse :type "/Game/Game/Blueprints/DamageSystem/Enum_DamageResponse Enum" :default "NewEnumerator0"))
  ;[1 0 0] Combat
  ;;[1 1 1] Damage and Death
  ;;;[1 1 1] Set Damage State
  (`KismetSystemLibrary.PrintString` "Is Hit")
  (`/Game/Game/Blueprints/Character/Enemy/AI/AIC_EnemyBase.SetStateAsHit` (`self.As AIC Enemy Base`))
  ;;;[1 1 1] Take Damage
  (`KismetSystemLibrary.Delay` 0.6)
  (`|PlayMontage` (`self.Mesh`) "/Game/Game/Blueprints/Animations/Montages/Montage_Ghoul_Hit.Montage_Ghoul_Hit"
    (:`then`
      (`GameplayStatics.PlaySoundAtLocation` "/Game/HumanVocalizations/HumanMaleB/Cues/voice_male_b_hurt_pain_set_5_16_Cue.voice_male_b_hurt_pain_set_5_16_Cue" (`self.K2_GetActorLocation`) (struct) 1.0 1.0 0.0 null null null null)
      ;;;[1 1 1] Set State to Attacking
      (`/Game/Game/Blueprints/Character/Enemy/AI/AIC_EnemyBase.SetStateAsAttacking` (`self.As AIC Enemy Base`) (`self.AttackTarget`))
      (`self.OnHitEnd`))))

(event `Death`
  (bind _returnvalue (`self.K2_GetActorLocation`))
  ;[1 0 0] Combat
  ;;[1 1 1] Damage and Death
  ;;;[1 1 1] Death Anim and Sound
  (set `self.bIsDead` true)
  (`/Game/Game/Blueprints/Character/Enemy/AI/AIC_EnemyBase.SetStateAsDead` (`self.As AIC Enemy Base`))
  (`PrimitiveComponent.SetCollisionEnabled` (`self.Mesh`) "NoCollision")
  (`KismetSystemLibrary.Delay` 0.6)
  (`|PlayMontage` (`self.Mesh`) "/Game/Game/Blueprints/Animations/Montages/Montage_Ghoul_Death.Montage_Ghoul_Death"
    (:`then`
      (`GameplayStatics.PlaySoundAtLocation` "/Game/HumanVocalizations/HumanMaleB/Cues/voice_male_b_death_low_02_Cue.voice_male_b_death_low_02_Cue" _returnvalue (struct) 1.0 1.0 0.0 null null null null)
      (`KismetSystemLibrary.Delay` 0.75)
      (bind _returnvalue_2 (`|SpawnActorFromClass` "/Game/ImproveFights_Vfx/Blueprints/BP_Explosion.BP_Explosion_C" (`KismetMathLibrary.MakeTransform` _returnvalue) "Undefined" "MultiplyWithRoot" null 1.0 0.25 "/Niagara/DefaultAssets/Templates/Systems/RadialBurst.RadialBurst" null))
      (`SceneComponent.SetHiddenInGame` (`self.Mesh`) false false)
      (`KismetSystemLibrary.Delay` 1.0)
      (`self.K2_DestroyActor` _returnvalue_2)
      (`self.K2_DestroyActor`))))

(event `Blocked`
  (params (bCanBeParried :type Boolean))
  ;[1 0 0] Combat
  ;;[1 1 1] Damage and Death
  (`KismetSystemLibrary.PrintString` "BLOCKED"))

(fn `DefaultAttackAI`
  ;[1 1 1] Execute Attack
  (`self.Punch`)
  (return))

(fn `GetCurrentHealth`
  (returns (Health :type "Float (double-precision)"))
  (return (`/Game/Game/Blueprints/DamageSystem/AC_DamageSystem_New.Health` (`self.AC_DamageSystem_New`))))

(fn `GetMaxHealth`
  (returns (MaxHealth :type "Float (double-precision)"))
  (return (`/Game/Game/Blueprints/DamageSystem/AC_DamageSystem_New.MaxHealth` (`self.AC_DamageSystem_New`))))

(fn `GetPatrolRoute`
  (returns (PatrolRoute :type "/Game/Game/Blueprints/Character/Enemy/BP_PatrolRoute Object Reference"))
  ;[1 1 1] Get Patrol Route
  (return (`self.PatrolRoute`)))

(fn `Heal`
  (params (HealAmount :type "Float (double-precision)"))
  (returns (NewHealth :type "Float (double-precision)"))
  (return 0.0))

(fn `TakeDamage`
  (params (DamageInfo :type "/Game/Game/Blueprints/DamageSystem/S_DamageInfo Structure"))
  (returns (bWasDamaged :type Boolean))
  (bind _bwasdamaged (`/Game/Game/Blueprints/DamageSystem/AC_DamageSystem_New.TakeDamage` (`self.AC_DamageSystem_New`) DamageInfo))
  (return _bwasdamaged))

(fn `UserConstructionScript`
  (bind _ac_damagesystem_new (`self.AC_DamageSystem_New`))
  ;[1 1 1] Bind BP_Ghoul to Event Dispatches in AC_DamageSystem
  (add `/Game/Game/Blueprints/DamageSystem/AC_DamageSystem_New.OnDeath` _ac_damagesystem_new (`|CreateDelegate` :!event `Death`))
  (add `/Game/Game/Blueprints/DamageSystem/AC_DamageSystem_New.OnDamageResponse` _ac_damagesystem_new (`|CreateDelegate` :!event `DamageResponse`)))