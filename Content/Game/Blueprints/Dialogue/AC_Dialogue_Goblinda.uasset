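; Dialogue component for Goblinda the Grocer, a nervous goblin NPC whose quest has the player buy her last Magic Node for 100 Money.
; The Dialogue override switches on ActiveDialogueBranch across quest offer, incomplete, turn-in and two post-quest conversations, chaining AddDialogue lines with options, voice cues and montages.
; Each ending sets the next branch and closes dialogue; the turn-in choice also sets TurnItIn.
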(fn `Dialogue`
  (bind _speaker (`self.Speaker`))
  (bind _speaker_2 (`self.Speaker`))
  (bind _speaker_3 (`self.Speaker`))
  (bind _speaker_4 (`self.Speaker`))
  (bind _speaker_5 (`self.Speaker`))
  ;[1 1 1] Begin Dialogue
  (`parent.Dialogue`)
  (set `self.Speaker` "Goblinda the Grocer")
  (switch `name` (`self.ActiveDialogueBranch`)
    (:`Default`
      (`KismetSystemLibrary.PrintString` "default is playing")
      ;[0 0 0] Assign Quest
      ;;[1 1 1] Hi
      (bind (_state _optionsindex) (`self.AddDialogue` _speaker "W-welcome to Goblart's Grocery! My name is Goblinda! How may I h-h-help you?" (`|MakeArray` "> Are you okay?" "> Why are you guys open?" "> Hello, Goblinda. How are you?" :!type "Text") :!label _label))
      (switch `/Game/Game/Blueprints/Dialogue/Enum_DialogueState` _state
        (:`NewEnumerator0`
          (switch `int` _optionsindex
            (:`0`
              _)
            (:`1`
              _)
            (:`2`
              _))
          ;;[1 1 1] Sneak supplies
          (bind (_state_2 _optionsindex_2) (`self.AddDialogue` _speaker "I didn't want to be out here, but my b-b-boss says we're short-staffed, and I can't leave the store alone." (`|MakeArray` "> Can I help at all?" "> Should I kill him?" "> You look really scared, dude." :!type "Text") "/Game/HumanVocalizations/HumanFemaleA/Cues/voice_female_a_expression_emote_sigh_Cue.voice_female_a_expression_emote_sigh_Cue" "/Game/Game/Blueprints/Animations/Montages/Montage_Goblin_Hit.Montage_Goblin_Hit"))
          (switch `/Game/Game/Blueprints/Dialogue/Enum_DialogueState` _state_2
            (:`NewEnumerator0`
              (switch `int` _optionsindex_2
                (:`0`
                  _)
                (:`1`
                  _)
                (:`2`
                  _))
              ;;[1 1 1] Can't afford
              (bind (_state_3 _optionsindex_3) (`self.AddDialogue` (`self.Speaker`) "I b-bet if sales were g-good enough, he wouldn't be mad if I closed early." (`|MakeArray` "> How much do you need?" :!type "Text") "/Game/HumanVocalizations/HumanFemaleA/Cues/voice_female_a_cry_11_Cue.voice_female_a_cry_11_Cue" "/Game/Game/Blueprints/Animations/Montages/Montage_Goblin_Hit.Montage_Goblin_Hit"))
              (switch `/Game/Game/Blueprints/Dialogue/Enum_DialogueState` _state_3
                (:`NewEnumerator0`
                  (switch `int` _optionsindex_3
                    (:`0`
                      ;;[1 1 1] Assign Quest
                      (bind (_state_4 _optionsindex_4) (`self.AddDialogue` (`self.Speaker`) "We have one Magic Node left. They're 100 Money. If I sell out, I bet I could go home. Do you want to buy it?" (`|MakeArray` "> I'll see what I can do." "> Maybe. No promises." "> Absolutely! I'll find the Money." :!type "Text") "/Game/HumanVocalizations/HumanFemaleA/Cues/voice_female_a_laugh_14_Cue.voice_female_a_laugh_14_Cue" "/Game/Game/Blueprints/Animations/Montages/Montage_Goblin_Hit.Montage_Goblin_Hit"))
                      (switch `/Game/Game/Blueprints/Dialogue/Enum_DialogueState` _state_4
                        (:`NewEnumerator0`
                          (switch `int` _optionsindex_4
                            (:`0`
                              _)
                            (:`1`
                              _)
                            (:`2`
                              _))
                          ;;[1 1 1] Promise reward
                          (bind (_state_5 _optionsindex_5) (`self.AddDialogue` (`self.Speaker`) "P-p-please come back soon. Have a fine shopping day!" (`|MakeArray` "> Bye!" :!type "Text") "/Game/HumanVocalizations/HumanFemaleA/Cues/voice_female_a_cry_11_Cue.voice_female_a_cry_11_Cue" "/Game/Game/Blueprints/Animations/Montages/Montage_Goblin_Hit.Montage_Goblin_Hit"))
                          (switch `/Game/Game/Blueprints/Dialogue/Enum_DialogueState` _state_5
                            (:`NewEnumerator0`
                              (switch `int` _optionsindex_5
                                (:`0`
                                  ;;[1 1 1] Set to Next Conversation
                                  (`self.SetDialogueBranch` "QuestIncomplete" "NewEnumerator1")
                                  ;;[1 1 1] Close Dialogue
                                  (`self.ClearDialogueProgress`)
                                  (`self.CloseDialogue`))))))))))))))))
    (:`AssignQuest`
      (goto _label))
    (:`QuestIncomplete`
      ;[0 0 0] QuestIncomplete
      ;;[1 1 1] Check-In
      (bind (_state_6 _optionsindex_6) (`self.AddDialogue` _speaker_3 "Welcome to G-G-Goblart's Grocery! I'm Goblinda. How may I help you? " (`|MakeArray` "> I'm just looking around." :!type "Text")))
      (switch `/Game/Game/Blueprints/Dialogue/Enum_DialogueState` _state_6
        (:`NewEnumerator0`
          (switch `int` _optionsindex_6
            (:`0`
              ;;[1 1 1] Proud of you
              (bind (_state_7 _optionsindex_7) (`self.AddDialogue` _speaker_3 "P-please enjoy our very fine wares. Thank you!" (`|MakeArray` "> Uh-huh. Thank you!" :!type "Text") "/Game/HumanVocalizations/HumanFemaleA/Cues/voice_female_a_expression_emote_sigh_Cue.voice_female_a_expression_emote_sigh_Cue" "/Game/Game/Blueprints/Animations/Montages/Montage_Goblin_Hit.Montage_Goblin_Hit"))
              (switch `/Game/Game/Blueprints/Dialogue/Enum_DialogueState` _state_7
                (:`NewEnumerator0`
                  (switch `int` _optionsindex_7
                    (:`0`
                      ;;[1 1 1] Set to Next Conversation
                      (`self.SetDialogueBranch` "QuestIncomplete" "NewEnumerator1")
                      ;;[1 1 1] Close Dialogue
                      (`self.ClearDialogueProgress`)
                      (`self.CloseDialogue`))))))))))
    (:`QuestComplete`
      ;[0 0 0] QuestComplete
      ;;[1 1 1] You did it!
      (bind (_state_8 _optionsindex_8) (`self.AddDialogue` _speaker_4 "Wel-Wel-Welcome to Goblart's Grocery! I'm terrified! I mean--I'm Goblinda! How may I help you?" (`|MakeArray` "> I would like to buy the Magic Node, please." :!type "Text")))
      (switch `/Game/Game/Blueprints/Dialogue/Enum_DialogueState` _state_8
        (:`NewEnumerator0`
          (switch `int` _optionsindex_8
            (:`0`
              ;;[1 1 1] Turn in?
              (bind (_state_9 _optionsindex_9) (`self.AddDialogue` _speaker_4 "Really?? You'll buy it? It's 100 Money. Is that okay?" (`|MakeArray` "> Yes, that's fine." "> Ah... That's too much." :!type "Text") "/Game/HumanVocalizations/HumanFemaleA/Cues/voice_female_a_laugh_14_Cue.voice_female_a_laugh_14_Cue" "/Game/Game/Blueprints/Animations/Montages/Montage_Goblin_Hit.Montage_Goblin_Hit"))
              (switch `/Game/Game/Blueprints/Dialogue/Enum_DialogueState` _state_9
                (:`NewEnumerator0`
                  (switch `int` _optionsindex_9
                    (:`0`
                      ;;[1 1 1] Yes Turn In
                      (bind (_state_10 _optionsindex_10) (`self.AddDialogue` _speaker_4 "You will? Really? Oh my gosh, thank you! That means we're sold out! I can go home." (`|MakeArray` "> Get out of here, kiddo!" :!type "Text") "/Game/HumanVocalizations/HumanFemaleA/Cues/voice_female_a_laugh_14_Cue.voice_female_a_laugh_14_Cue" "/Game/UndeadPack/EnemyGoblin/Animations/Anim_Arg_Montage.Anim_Arg_Montage"))
                      (switch `/Game/Game/Blueprints/Dialogue/Enum_DialogueState` _state_10
                        (:`NewEnumerator0`
                          (switch `int` _optionsindex_10
                            (:`0`
                              ;;[1 1 1] Reward
                              (bind (_state_11 _optionsindex_11) (`self.AddDialogue` _speaker_4 "I seriously owe you so much. Okay, I'll take the Money, and here's the Magic Node! Thank you!!" (`|MakeArray` "> Get home safe, Goblinda!" :!type "Text") "/Game/HumanVocalizations/HumanFemaleA/Cues/voice_female_a_laugh_14_Cue.voice_female_a_laugh_14_Cue" "/Game/Game/Blueprints/Animations/Montages/Montage_Goblin_Hit.Montage_Goblin_Hit"))
                              (switch `/Game/Game/Blueprints/Dialogue/Enum_DialogueState` _state_11
                                (:`NewEnumerator0`
                                  (switch `int` _optionsindex_11
                                    (:`0`
                                      ;;[1 1 1] Finish Quest
                                      (`self.SetDialogueBranch` "AfterQuest1" "NewEnumerator1")
                                      (set `self.bTurnItIn?` true))))))))))
                    (:`1`
                      ;;[1 1 1] No Don't Turn In
                      (bind (_state_12 _optionsindex_12) (`self.AddDialogue` _speaker_4 "O-oh. Of c-c-course. I'll just... Keep minding the store. During an undead invasion. If I can help you with anything, p-p-please let me know." (`|MakeArray` "> Thank you." :!type "Text") "/Game/HumanVocalizations/HumanFemaleA/Cues/voice_female_a_expression_emote_sigh_Cue.voice_female_a_expression_emote_sigh_Cue" "/Game/Game/Blueprints/Animations/Montages/Montage_Goblin_Hit.Montage_Goblin_Hit"))
                      (switch `/Game/Game/Blueprints/Dialogue/Enum_DialogueState` _state_12
                        (:`NewEnumerator0`
                          (switch `int` _optionsindex_12
                            (:`0`
                              (`self.SetDialogueBranch` "QuestComplete" "NewEnumerator1")
                              (set `self.bTurnItIn?` false)))))))
                  ;;[1 1 1] Close Dialogue
                  (`self.ClearDialogueProgress`)
                  (`self.CloseDialogue`))))))))
    (:`AfterQuest1`
      ;[0 0 0] AfterQuest1
      ;;[1 1 1] Thanks
      (bind (_state_13 _optionsindex_13) (`self.AddDialogue` _speaker_2 "I'm so excited. As soon as I finish sweeping up, I'm out of here!" (`|MakeArray` "> Don't sweep. Go home!" :!type "Text")))
      (switch `/Game/Game/Blueprints/Dialogue/Enum_DialogueState` _state_13
        (:`NewEnumerator0`
          (switch `int` _optionsindex_13
            (:`0`
              ;;[1 1 1] Closer as friends
              (bind (_state_14 _optionsindex_14) (`self.AddDialogue` _speaker_2 "Oh, haha. I c-can't afford to lose this job. But I'll go home as soon as I can!" (`|MakeArray` "> Keep safe!" :!type "Text") "/Game/HumanVocalizations/HumanFemaleA/Cues/voice_female_a_cry_11_Cue.voice_female_a_cry_11_Cue" "/Game/Game/Blueprints/Animations/Montages/Montage_Goblin_Hit.Montage_Goblin_Hit"))
              (switch `/Game/Game/Blueprints/Dialogue/Enum_DialogueState` _state_14
                (:`NewEnumerator0`
                  (switch `int` _optionsindex_14
                    (:`0`
                      ;;[1 1 1] Set to Next Conversation
                      (`self.SetDialogueBranch` "AfterQuest2" "NewEnumerator1")
                      ;;[1 1 1] Close Dialogue
                      (`self.ClearDialogueProgress`)
                      (`self.CloseDialogue`))))))))))
    (:`AfterQuest2`
      ;[0 0 0] AfterQuest2
      ;;[1 1 1] Thanks
      (bind (_state_15 _optionsindex_15) (`self.AddDialogue` _speaker_5 "Almost done! It's so scary walking home with ghouls leering at you. " (`|MakeArray` "> Are you going to be okay?" :!type "Text") "/Game/HumanVocalizations/HumanFemaleA/Cues/voice_female_a_effort_tired_01_Cue.voice_female_a_effort_tired_01_Cue"))
      (switch `/Game/Game/Blueprints/Dialogue/Enum_DialogueState` _state_15
        (:`NewEnumerator0`
          (switch `int` _optionsindex_15
            (:`0`
              ;;[1 1 1] Closer as friends
              (bind (_state_16 _optionsindex_16) (`self.AddDialogue` _speaker_5 "Haha! Probably not. Oh! But I'll get home alright, if that's what you mean." (`|MakeArray` "> Keep safe!" :!type "Text") "/Game/HumanVocalizations/HumanFemaleA/Cues/voice_female_a_laugh_14_Cue.voice_female_a_laugh_14_Cue" "/Game/Game/Blueprints/Animations/Montages/Montage_Goblin_Hit.Montage_Goblin_Hit"))
              (switch `/Game/Game/Blueprints/Dialogue/Enum_DialogueState` _state_16
                (:`NewEnumerator0`
                  (switch `int` _optionsindex_16
                    (:`0`
                      ;;[1 1 1] Set to Next Conversation
                      (`self.SetDialogueBranch` "AfterQuest2" "NewEnumerator1")
                      ;;[1 1 1] Close Dialogue
                      (`self.ClearDialogueProgress`)
                      (`self.CloseDialogue`))))))))))))