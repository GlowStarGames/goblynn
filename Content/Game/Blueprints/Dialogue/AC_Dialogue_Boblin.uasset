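; Dialogue component for Boblin the Tavernkeeper, whose quest asks Goblynn to donate Money for supplies in return for a Magic Node.
; The Dialogue override switches on ActiveDialogueBranch across quest assignment, incomplete, turn-in and two post-quest stages, with unmatched branches falling back to assignment.
; Chained AddDialogue calls supply lines, options, voice cues and montages.
; Endings save the next branch and close dialogue; the turn-in choice also sets TurnItIn.
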(fn `Dialogue`
  (bind _speaker (`self.Speaker`))
  (bind _speaker_2 (`self.Speaker`))
  (bind _speaker_3 (`self.Speaker`))
  (bind _speaker_4 (`self.Speaker`))
  (bind _speaker_5 (`self.Speaker`))
  ;[1 1 1] Begin Dialogue
  (`parent.Dialogue`)
  (set `self.Speaker` "Boblin the Tavernkeeper")
  (switch `name` (`self.ActiveDialogueBranch`)
    (:`Default`
      ;[0 0 0] Assign Quest
      ;;[1 1 1] Hi
      (bind (_state _optionsindex) (`self.AddDialogue` _speaker "Hey, Goblynn!" (`|MakeArray` "> Boblin! Hey!" :!type "Text") :!label _label))
      (switch `/Game/Game/Blueprints/Dialogue/Enum_DialogueState` _state
        (:`NewEnumerator0`
          (switch `int` _optionsindex
            (:`0`
              ;;[1 1 1] Sneak supplies
              (bind (_state_2 _optionsindex_2) (`self.AddDialogue` _speaker "People are too scared to leave their homes, so I'm trying to sneak supplies around to everyone." (`|MakeArray` "> Need help?" "> That's badass, dude." "> Boblin, that's dangerous!" :!type "Text") "/Game/HumanVocalizations/HumanMaleB/Cues/voice_male_b_breath_sigh_04_Cue.voice_male_b_breath_sigh_04_Cue" "/Game/Game/Blueprints/Animations/Montages/Montage_Goblin_Hit.Montage_Goblin_Hit"))
              (switch `/Game/Game/Blueprints/Dialogue/Enum_DialogueState` _state_2
                (:`NewEnumerator0`
                  (switch `int` _optionsindex_2
                    (:`0`
                      _)
                    (:`1`
                      _)
                    (:`2`
                      _))
                  ;;[1 1 1] Can't afford
                  (bind (_state_3 _optionsindex_3) (`self.AddDialogue` (`self.Speaker`) "Some of the merchants are price-gouging. I can't afford all the supplies I need." (`|MakeArray` "> You need money?" "> Should I kill them?" "> That's so unfair!" :!type "Text") "/Game/HumanVocalizations/HumanMaleB/Cues/voice_male_b_breath_sigh_02_Cue.voice_male_b_breath_sigh_02_Cue" "/Game/Game/Blueprints/Animations/Montages/Montage_Goblin_Hit.Montage_Goblin_Hit"))
                  (switch `/Game/Game/Blueprints/Dialogue/Enum_DialogueState` _state_3
                    (:`NewEnumerator0`
                      (switch `int` _optionsindex_3
                        (:`0`
                          _)
                        (:`1`
                          _)
                        (:`2`
                          _))
                      ;;[1 1 1] Assign Quest
                      (bind (_state_4 _optionsindex_4) (`self.AddDialogue` (`self.Speaker`) "Can you just... Can you spare, like, 100 Money? Just enough to get everybody fed for now." (`|MakeArray` "> I'll see what I can do." "> Maybe. No promises." "> Absolutely! I'll get the Money!" :!type "Text") "/Game/HumanVocalizations/HumanMaleB/Cues/voice_male_b_breath_sigh_04_Cue.voice_male_b_breath_sigh_04_Cue" "/Game/Game/Blueprints/Animations/Montages/Montage_Goblin_Hit.Montage_Goblin_Hit"))
                      (switch `/Game/Game/Blueprints/Dialogue/Enum_DialogueState` _state_4
                        (:`NewEnumerator0`
                          (switch `int` _optionsindex_4
                            (:`0`
                              _)
                            (:`1`
                              _)
                            (:`2`
                              _))
                          ;;[1 1 1] Promise reward
                          (bind (_state_5 _optionsindex_5) (`self.AddDialogue` (`self.Speaker`) "Thanks, Goblynn. If you can get me the Money, I'll help you out too." (`|MakeArray` "> Hang in there, Boblin." :!type "Text") "/Game/HumanVocalizations/HumanMaleB/Cues/voice_male_b_breath_sigh_02_Cue.voice_male_b_breath_sigh_02_Cue" "/Game/Game/Blueprints/Animations/Montages/Montage_Goblin_Hit.Montage_Goblin_Hit"))
                          (switch `/Game/Game/Blueprints/Dialogue/Enum_DialogueState` _state_5
                            (:`NewEnumerator0`
                              (switch `int` _optionsindex_5
                                (:`0`
                                  ;;[1 1 1] Set to Next Conversation
                                  (`self.SetDialogueBranch` "QuestIncomplete" "NewEnumerator1")
                                  ;;[1 1 1] Close Dialogue
                                  (`self.ClearDialogueProgress`)
                                  (`self.CloseDialogue`))))))))))))))))
    (:`AssignQuest`
      (goto _label))
    (:`QuestIncomplete`
      ;[0 0 0] QuestIncomplete
      ;;[1 1 1] Check-In
      (bind (_state_6 _optionsindex_6) (`self.AddDialogue` _speaker_3 "Goblynn! Do you have the Money?" (`|MakeArray` "> Not yet." :!type "Text")))
      (switch `/Game/Game/Blueprints/Dialogue/Enum_DialogueState` _state_6
        (:`NewEnumerator0`
          (switch `int` _optionsindex_6
            (:`0`
              ;;[1 1 1] Proud of you
              (bind (_state_7 _optionsindex_7) (`self.AddDialogue` _speaker_3 "Please hurry. Most people are too scared to go out and get food on their own. They're counting on us." (`|MakeArray` "> I'll be back." :!type "Text") "/Game/HumanVocalizations/HumanMaleB/Cues/voice_male_b_breath_sigh_02_Cue.voice_male_b_breath_sigh_02_Cue" "/Game/Game/Blueprints/Animations/Montages/Montage_Goblin_Hit.Montage_Goblin_Hit"))
              (switch `/Game/Game/Blueprints/Dialogue/Enum_DialogueState` _state_7
                (:`NewEnumerator0`
                  (switch `int` _optionsindex_7
                    (:`0`
                      ;;[1 1 1] Set to Next Conversation
                      (`self.SetDialogueBranch` "QuestIncomplete" "NewEnumerator1")
                      ;;[1 1 1] Close Dialogue
                      (`self.ClearDialogueProgress`)
                      (`self.CloseDialogue`))))))))))
    (:`QuestComplete`
      ;[0 0 0] QuestComplete
      ;;[1 1 1] You did it!
      (bind (_state_8 _optionsindex_8) (`self.AddDialogue` _speaker_4 "Hey! Any luck?" (`|MakeArray` "> I have the money!" :!type "Text")))
      (switch `/Game/Game/Blueprints/Dialogue/Enum_DialogueState` _state_8
        (:`NewEnumerator0`
          (switch `int` _optionsindex_8
            (:`0`
              ;;[1 1 1] Turn in?
              (bind (_state_9 _optionsindex_9) (`self.AddDialogue` _speaker_4 "Fantastic! So you'll donate 100 Money?" (`|MakeArray` "> Yes! Here you go." "> Hold on. I may still need it." :!type "Text") "/Game/HumanVocalizations/HumanMaleB/Cues/voice_male_b_laugh_short_07_Cue.voice_male_b_laugh_short_07_Cue" "/Game/Game/Blueprints/Animations/Montages/Montage_Goblin_Hit.Montage_Goblin_Hit"))
              (switch `/Game/Game/Blueprints/Dialogue/Enum_DialogueState` _state_9
                (:`NewEnumerator0`
                  (switch `int` _optionsindex_9
                    (:`0`
                      ;;[1 1 1] Yes Turn In
                      (bind (_state_10 _optionsindex_10) (`self.AddDialogue` _speaker_4 "That's fantastic! Thank you! " (`|MakeArray` "> Of course!" :!type "Text") "/Game/HumanVocalizations/HumanMaleB/Cues/voice_male_b_laugh_intense_01_Cue.voice_male_b_laugh_intense_01_Cue" "/Game/UndeadPack/EnemyGoblin/Animations/Anim_Arg_Montage.Anim_Arg_Montage"))
                      (switch `/Game/Game/Blueprints/Dialogue/Enum_DialogueState` _state_10
                        (:`NewEnumerator0`
                          (switch `int` _optionsindex_10
                            (:`0`
                              ;;[1 1 1] Reward
                              (bind (_state_11 _optionsindex_11) (`self.AddDialogue` _speaker_4 "Here, take this Magic Node. I stole it from one of the undead who tried to catch me. I hope it helps!" (`|MakeArray` "> Thanks, Boblin!" :!type "Text") "/Game/HumanVocalizations/HumanMaleB/Cues/voice_male_b_laugh_short_07_Cue.voice_male_b_laugh_short_07_Cue" "/Game/Game/Blueprints/Animations/Montages/Montage_Goblin_Hit.Montage_Goblin_Hit"))
                              (switch `/Game/Game/Blueprints/Dialogue/Enum_DialogueState` _state_11
                                (:`NewEnumerator0`
                                  (switch `int` _optionsindex_11
                                    (:`0`
                                      ;;[1 1 1] Finish Quest
                                      (`self.SetDialogueBranch` "AfterQuest1" "NewEnumerator1")
                                      (set `self.bTurnItIn?` true))))))))))
                    (:`1`
                      ;;[1 1 1] No Don't Turn In
                      (bind (_state_12 _optionsindex_12) (`self.AddDialogue` _speaker_4 "People need that Money, Goblynn. I can't hide out here forever." (`|MakeArray` "> I know." :!type "Text") "/Game/HumanVocalizations/HumanMaleB/Cues/voice_male_b_breath_sigh_04_Cue.voice_male_b_breath_sigh_04_Cue" "/Game/Game/Blueprints/Animations/Montages/Montage_Goblin_Hit.Montage_Goblin_Hit"))
                      (switch `/Game/Game/Blueprints/Dialogue/Enum_DialogueState` _state_12
                        (:`NewEnumerator0`
                          (switch `int` _optionsindex_12
                            (:`0`
                              (`self.SetDialogueBranch` "QuestComplete" "NewEnumerator1")
                              (set `self.bTurnItIn?` false)))))))
                  ;;[1 1 1] Close Dialogue
                  (`self.ClearDialogueProgress`)
                  (`self.CloseDialogue`))))))))
    (:`AfterQuest1`
      ;[0 0 0] AfterQuest1
      ;;[1 1 1] Thanks
      (bind (_state_13 _optionsindex_13) (`self.AddDialogue` _speaker_5 "Thanks to you, I was able to get some infant formula over to the Hobbes family" (`|MakeArray` "> Great work, Boblin!" :!type "Text")))
      (switch `/Game/Game/Blueprints/Dialogue/Enum_DialogueState` _state_13
        (:`NewEnumerator0`
          (switch `int` _optionsindex_13
            (:`0`
              ;;[1 1 1] Closer as friends
              (bind (_state_14 _optionsindex_14) (`self.AddDialogue` _speaker_5 "Ah ah! Call me Bob. We're friends now, Lynn." (`|MakeArray` "> Great work, Bob!" :!type "Text") "/Game/HumanVocalizations/HumanMaleB/Cues/voice_male_b_laugh_short_07_Cue.voice_male_b_laugh_short_07_Cue" "/Game/Game/Blueprints/Animations/Montages/Montage_Goblin_Hit.Montage_Goblin_Hit"))
              (switch `/Game/Game/Blueprints/Dialogue/Enum_DialogueState` _state_14
                (:`NewEnumerator0`
                  (switch `int` _optionsindex_14
                    (:`0`
                      ;;[1 1 1] Set to Next Conversation
                      (`self.SetDialogueBranch` "AfterQuest2" "NewEnumerator1")
                      ;;[1 1 1] Close Dialogue
                      (`self.ClearDialogueProgress`)
                      (`self.CloseDialogue`))))))))))
    (:`AfterQuest2`
      ;[0 0 0] AfterQuest2
      ;;[1 1 1] Thanks
      (set `self.Speaker` "Bob the Tavernkeeper")
      (bind (_state_15 _optionsindex_15) (`self.AddDialogue` _speaker_2 "Everyone should make it tonight, but if this keeps up, we're going to have to do something about the price-gouging." (`|MakeArray` "> We'll have to organize something." :!type "Text")))
      (switch `/Game/Game/Blueprints/Dialogue/Enum_DialogueState` _state_15
        (:`NewEnumerator0`
          (switch `int` _optionsindex_15
            (:`0`
              ;;[1 1 1] Closer as friends
              (bind (_state_16 _optionsindex_16) (`self.AddDialogue` _speaker_2 "We'll discuss it later. Good luck, Lynn." (`|MakeArray` "> You too, Bob!" :!type "Text") "/Game/HumanVocalizations/HumanMaleB/Cues/voice_male_b_breath_sigh_02_Cue.voice_male_b_breath_sigh_02_Cue" "/Game/Game/Blueprints/Animations/Montages/Montage_Goblin_Hit.Montage_Goblin_Hit"))
              (switch `/Game/Game/Blueprints/Dialogue/Enum_DialogueState` _state_16
                (:`NewEnumerator0`
                  (switch `int` _optionsindex_16
                    (:`0`
                      ;;[1 1 1] Set to Next Conversation
                      (`self.SetDialogueBranch` "AfterQuest2" "NewEnumerator1")
                      ;;[1 1 1] Close Dialogue
                      (`self.ClearDialogueProgress`)
                      (`self.CloseDialogue`))))))))))))