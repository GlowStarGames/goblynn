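; Dialogue component for the NPC Goblanche the Veteran, whose quest trades a Magic Node for blowing up an undead supply cart and a way onto the wall.
; Dialogue overrides the parent and switches on ActiveDialogueBranch through quest offer, incomplete, turn-in and two after-quest chats.
; AddDialogue chains supply lines, options, voice cues and montages; endings save the next branch and close.
; Turn-in sets TurnItIn, leaving the actual reward and explosion outside this graph.
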(fn `Dialogue`
  (bind _speaker (`self.Speaker`))
  (bind _speaker_2 (`self.Speaker`))
  (bind _speaker_3 (`self.Speaker`))
  (bind _speaker_4 (`self.Speaker`))
  (bind _speaker_5 (`self.Speaker`))
  ;[1 1 1] Begin Dialogue
  (`parent.Dialogue`)
  (set `self.Speaker` "Goblanche the Veteran")
  (switch `name` (`self.ActiveDialogueBranch`)
    (:`Default`
      ;[0 0 0] Assign Quest
      ;;[1 1 1] Hi
      (bind (_state _optionsindex) (`self.AddDialogue` _speaker "Hey there, kiddo. You're out and about in a dangerous time." (`|MakeArray` "> I sure am. Weird times." "> You're one to talk." "> I can handle myself okay!" :!type "Text") :!label _label))
      (switch `/Game/Game/Blueprints/Dialogue/Enum_DialogueState` _state
        (:`NewEnumerator0`
          (switch `int` _optionsindex
            (:`0`
              _)
            (:`1`
              _)
            (:`2`
              _))
          ;;[1 1 1] Sneak supplies
          (bind (_state_2 _optionsindex_2) (`self.AddDialogue` _speaker "I've been fighting the Lich Emperor's undead army my whole life. This is how it goes." (`|MakeArray` "> What should we do?" "> You sound resigned." "> So you've seen this before?" :!type "Text") "/Game/HumanVocalizations/HumanFemaleA/Cues/voice_female_a_breath_tired_01_Cue.voice_female_a_breath_tired_01_Cue" "/Game/Game/Blueprints/Animations/Montages/Montage_Goblin_Hit.Montage_Goblin_Hit"))
          (switch `/Game/Game/Blueprints/Dialogue/Enum_DialogueState` _state_2
            (:`NewEnumerator0`
              (switch `int` _optionsindex_2
                (:`0`
                  _)
                (:`1`
                  _)
                (:`2`
                  _))
              ;;[1 1 1] Can't afford
              (bind (_state_3 _optionsindex_3) (`self.AddDialogue` (`self.Speaker`) "I may be tired, but I still have some tricks up my sleeve. There's a giant supply cart on the corner, at the end of the water. It's full of magic shit." (`|MakeArray` "> So?" :!type "Text") "/Game/HumanVocalizations/HumanFemaleA/Cues/voice_female_a_breath_tired_01_Cue.voice_female_a_breath_tired_01_Cue" "/Game/Game/Blueprints/Animations/Montages/Montage_Goblin_Hit.Montage_Goblin_Hit"))
              (switch `/Game/Game/Blueprints/Dialogue/Enum_DialogueState` _state_3
                (:`NewEnumerator0`
                  (switch `int` _optionsindex_3
                    (:`0`
                      ;;[1 1 1] Assign Quest
                      (bind (_state_4 _optionsindex_4) (`self.AddDialogue` (`self.Speaker`) "So if you get me a Magic Node, I can overload all that magic. Blow up their supplies." (`|MakeArray` "> Whoa! I'll see what I can do." "> Maybe. I need Magic Nodes too." "> I want to see that! I'll get you one." :!type "Text") "/Game/HumanVocalizations/HumanFemaleA/Cues/voice_female_a_expression_emote_04_Cue.voice_female_a_expression_emote_04_Cue" "/Game/Game/Blueprints/Animations/Montages/Montage_Goblin_Hit.Montage_Goblin_Hit"))
                      (switch `/Game/Game/Blueprints/Dialogue/Enum_DialogueState` _state_4
                        (:`NewEnumerator0`
                          (switch `int` _optionsindex_4
                            (:`0`
                              _)
                            (:`1`
                              _)
                            (:`2`
                              _))
                          ;;[1 1 1] Promise reward
                          (bind (_state_5 _optionsindex_5) (`self.AddDialogue` (`self.Speaker`) "You're a good kid. I understand if you can't spare it. But if you can get me a Magic Node, I'll help you get up on that wall. " (`|MakeArray` "> Oh? I'll think about that, Mx. Goblanche!" :!type "Text") "/Game/HumanVocalizations/HumanFemaleA/Cues/voice_female_a_expression_emote_04_Cue.voice_female_a_expression_emote_04_Cue" "/Game/Game/Blueprints/Animations/Montages/Montage_Goblin_Hit.Montage_Goblin_Hit"))
                          (switch `/Game/Game/Blueprints/Dialogue/Enum_DialogueState` _state_5
                            (:`NewEnumerator0`
                              (switch `int` _optionsindex_5
                                (:`0`
                                  ;;[1 1 1] Set to Next Conversation
                                  (`self.SetDialogueBranch` "QuestIncomplete" "NewEnumerator1")
                                  ;;[1 1 1] Close Dialogue
                                  (`self.ClearDialogueProgress`)
                                  (`self.CloseDialogue`))))))))))))))))
    (:`AssignQuest`
      (goto _label))
    (:`QuestIncomplete`
      ;[0 0 0] QuestIncomplete
      ;;[1 1 1] Check-In
      (bind (_state_6 _optionsindex_6) (`self.AddDialogue` _speaker_3 "Hey, kiddo. You got a Magic Node for me?" (`|MakeArray` "> Not yet." :!type "Text")))
      (switch `/Game/Game/Blueprints/Dialogue/Enum_DialogueState` _state_6
        (:`NewEnumerator0`
          (switch `int` _optionsindex_6
            (:`0`
              ;;[1 1 1] Proud of you
              (bind (_state_7 _optionsindex_7) (`self.AddDialogue` _speaker_3 "Bring me something fun, and we can ruin their day. Or their night. Whatever. " (`|MakeArray` "> I'll think about it, Mx. Goblanche!" :!type "Text") "/Game/HumanVocalizations/HumanFemaleA/Cues/voice_female_a_expression_emote_04_Cue.voice_female_a_expression_emote_04_Cue" "/Game/Game/Blueprints/Animations/Montages/Montage_Goblin_Hit.Montage_Goblin_Hit"))
              (switch `/Game/Game/Blueprints/Dialogue/Enum_DialogueState` _state_7
                (:`NewEnumerator0`
                  (switch `int` _optionsindex_7
                    (:`0`
                      ;;[1 1 1] Set to Next Conversation
                      (`self.SetDialogueBranch` "QuestIncomplete" "NewEnumerator1")
                      ;;[1 1 1] Close Dialogue
                      (`self.ClearDialogueProgress`)
                      (`self.CloseDialogue`))))))))))
    (:`QuestComplete`
      ;[0 0 0] QuestComplete
      ;;[1 1 1] You did it!
      (bind (_state_8 _optionsindex_8) (`self.AddDialogue` _speaker_4 "Well, well, it's Goblynn! You got something fun for me?" (`|MakeArray` "> I found a Magic Node!" :!type "Text")))
      (switch `/Game/Game/Blueprints/Dialogue/Enum_DialogueState` _state_8
        (:`NewEnumerator0`
          (switch `int` _optionsindex_8
            (:`0`
              ;;[1 1 1] Turn in?
              (bind (_state_9 _optionsindex_9) (`self.AddDialogue` _speaker_4 "Well done, kiddo. You ready to wreck some shit? I'll need the Magic Node." (`|MakeArray` "> Hell yes. Here you go!" "> On second thought..." :!type "Text") "/Game/HumanVocalizations/HumanFemaleA/Cues/voice_female_a_breath_tired_01_Cue.voice_female_a_breath_tired_01_Cue" "/Game/Game/Blueprints/Animations/Montages/Montage_Goblin_Hit.Montage_Goblin_Hit"))
              (switch `/Game/Game/Blueprints/Dialogue/Enum_DialogueState` _state_9
                (:`NewEnumerator0`
                  (switch `int` _optionsindex_9
                    (:`0`
                      ;;[1 1 1] Yes Turn In
                      (bind (_state_10 _optionsindex_10) (`self.AddDialogue` _speaker_4 "That's perfect. Here's a little tip for your trouble. 30 Money for a job well done." (`|MakeArray` "> Whoa, thanks Mx. Goblanche!" :!type "Text") "/Game/HumanVocalizations/HumanFemaleA/Cues/voice_female_a_expression_emote_04_Cue.voice_female_a_expression_emote_04_Cue" "/Game/Game/Blueprints/Animations/Montages/Montage_Goblin_Hit.Montage_Goblin_Hit"))
                      (switch `/Game/Game/Blueprints/Dialogue/Enum_DialogueState` _state_10
                        (:`NewEnumerator0`
                          (switch `int` _optionsindex_10
                            (:`0`
                              ;;[1 1 1] Reward
                              (bind (_state_11 _optionsindex_11) (`self.AddDialogue` _speaker_4 "Now are you ready for this explosion? Stand back!" (`|MakeArray` "> Alright!!" :!type "Text") "/Game/HumanVocalizations/HumanFemaleA/Cues/voice_female_a_battle_shout_03_Cue.voice_female_a_battle_shout_03_Cue" "/Game/UndeadPack/EnemyGoblin/Animations/Anim_Attack1_Montage.Anim_Attack1_Montage"))
                              (switch `/Game/Game/Blueprints/Dialogue/Enum_DialogueState` _state_11
                                (:`NewEnumerator0`
                                  (switch `int` _optionsindex_11
                                    (:`0`
                                      ;;[1 1 1] Finish Quest
                                      (`self.SetDialogueBranch` "AfterQuest1" "NewEnumerator1")
                                      (set `self.bTurnItIn?` true))))))))))
                    (:`1`
                      ;;[1 1 1] No Don't Turn In
                      (bind (_state_12 _optionsindex_12) (`self.AddDialogue` _speaker_4 "Hey, that's okay. But if you ever want to stick it to those undead bastards, I'll be here." (`|MakeArray` "> Right on." :!type "Text") "/Game/HumanVocalizations/HumanFemaleA/Cues/voice_female_a_breath_tired_01_Cue.voice_female_a_breath_tired_01_Cue" "/Game/Game/Blueprints/Animations/Montages/Montage_Goblin_Hit.Montage_Goblin_Hit"))
                      (switch `/Game/Game/Blueprints/Dialogue/Enum_DialogueState` _state_12
                        (:`NewEnumerator0`
                          (switch `int` _optionsindex_12
                            (:`0`
                              (`self.SetDialogueBranch` "QuestComplete" "NewEnumerator1")
                              (set `self.bTurnItIn?` false)))))))
                  ;;[1 1 1] Close Dialogue
                  (`self.ClearDialogueProgress`)
                  (`self.CloseDialogue`))))))))
    (:`AfterQuest1`
      ;[0 0 0] AfterQuest1
      ;;[1 1 1] Thanks
      (bind (_state_13 _optionsindex_13) (`self.AddDialogue` _speaker_5 "Haha!  Bet you didn't know a Magic Node could do that!" (`|MakeArray` "> Can you teach me??" :!type "Text")))
      (switch `/Game/Game/Blueprints/Dialogue/Enum_DialogueState` _state_13
        (:`NewEnumerator0`
          (switch `int` _optionsindex_13
            (:`0`
              ;;[1 1 1] Closer as friends
              (bind (_state_14 _optionsindex_14) (`self.AddDialogue` _speaker_5 "Not tonight, kiddo. But there's a big pile of wood left over after the explosion. I bet you could use it to climb up onto the wall!" (`|MakeArray` "> Thanks, Mx. Goblanche!" :!type "Text") "/Game/HumanVocalizations/HumanFemaleA/Cues/voice_female_a_battle_shout_03_Cue.voice_female_a_battle_shout_03_Cue" "/Game/UndeadPack/EnemyGoblin/Animations/Anim_Arg_Montage.Anim_Arg_Montage"))
              (switch `/Game/Game/Blueprints/Dialogue/Enum_DialogueState` _state_14
                (:`NewEnumerator0`
                  (switch `int` _optionsindex_14
                    (:`0`
                      ;;[1 1 1] Set to Next Conversation
                      (`self.SetDialogueBranch` "AfterQuest2" "NewEnumerator1")
                      ;;[1 1 1] Close Dialogue
                      (`self.ClearDialogueProgress`)
                      (`self.CloseDialogue`))))))))))
    (:`AfterQuest2`
      ;[0 0 0] AfterQuest2
      ;;[1 1 1] Thanks
      (bind (_state_15 _optionsindex_15) (`self.AddDialogue` _speaker_2 "Boy, I'm tired.That tuckered me out." (`|MakeArray` "> I'll take it from here, Mx. Goblanche!" :!type "Text")))
      (switch `/Game/Game/Blueprints/Dialogue/Enum_DialogueState` _state_15
        (:`NewEnumerator0`
          (switch `int` _optionsindex_15
            (:`0`
              ;;[1 1 1] Closer as friends
              (bind (_state_16 _optionsindex_16) (`self.AddDialogue` _speaker_2 "Haha! You're a good kid. You gone exploring on that wall yet?" (`|MakeArray` "> Talk to you later!" :!type "Text") "/Game/HumanVocalizations/HumanFemaleA/Cues/voice_female_a_breath_tired_01_Cue.voice_female_a_breath_tired_01_Cue" "/Game/Game/Blueprints/Animations/Montages/Montage_Goblin_Hit.Montage_Goblin_Hit"))
              (switch `/Game/Game/Blueprints/Dialogue/Enum_DialogueState` _state_16
                (:`NewEnumerator0`
                  (switch `int` _optionsindex_16
                    (:`0`
                      ;;[1 1 1] Set to Next Conversation
                      (`self.SetDialogueBranch` "AfterQuest2" "NewEnumerator1")
                      ;;[1 1 1] Close Dialogue
                      (`self.ClearDialogueProgress`)
                      (`self.CloseDialogue`))))))))))))