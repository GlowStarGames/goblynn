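; Base dialogue component that shows WBP_Dialogue lines with optional audio and montages on its owner, async-loading unloaded assets.
; Child classes script conversations in the empty Dialogue function through AddDialogue calls.
; Each selection is saved by index and Dialogue reruns from the start, skipping answered lines to show the next one.
; Branch switching stores or clears the current branch's progress, then restores the target's.
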(event `self.ReceiveBeginPlay`
  ;[1 1 1] Create Audio Component if using audio
  (if (`self.bUseAudio?`)
    (bind _returnvalue (`|AddComponentByClass` :`self` (`self.GetOwner`) :`Class` "/Script/Engine.AudioComponent"))
    (set `self.AudioComponent` _returnvalue)
    (set `self.bTurnItIn?` false)))

(event `LoadDialogueAudio`
  (params (SoundBase :type "SoundBase Soft Object Reference"))
  (bind _audiocomponent (`self.AudioComponent`))
  ;[1 1 1] Async Load Dialogue Audio
  (bind _object (`|LoadAsset` SoundBase)
    (:`Completed`
      (bind _assound_base (cast `SoundBase` _object))
      (`AudioComponent.SetSound` _audiocomponent _assound_base)
      (`AudioComponent.Play` _audiocomponent 0.0))))

(event `PlayAnimation`
  (params (MontageToPlay :type "AnimMontage Soft Object Reference"))
  (bind _output (`|ConvertAsset` MontageToPlay))
  ;[1 1 1] Async Load Animation
  ;;[1 1 1] Call Valid Montage
  (`/Engine/EditorBlueprintResources/StandardMacros.IsValid` _output
    (:`Is Valid`
      (`self.PlayLoadedMontage` _output))
    (:`Is Not Valid`
      ;;[1 1 1] Load Invalid Montage
      (bind _object (`|LoadAsset` MontageToPlay)
        (:`Completed`
          (bind _asanim_montage (cast `AnimMontage` _object))
          (`self.PlayLoadedMontage` _asanim_montage))))))

(event `PlayLoadedMontage`
  (params (Montage :type "AnimMontage Object Reference"))
  ;[1 1 1] Play Animation
  (`|PlayMontage` (`Actor.GetComponentByClass` (`self.GetOwner`) "/Script/Engine.SkeletalMeshComponent") Montage))

(fn `AddDialogue`
  (params (Speaker :type Text) (Dialogue :type Text) (OptionsText :type "Array of Text") (DialogueAudio :type "SoundBase Soft Object Reference") (Animation :type "AnimMontage Soft Object Reference"))
  (returns (State :type "/Game/Game/Blueprints/Dialogue/Enum_DialogueState Enum") (OptionsIndex :type Integer))
  (bind (_value _returnvalue) (`BlueprintMapLibrary.Map_Find` (`self.DialogueProgress`) (`self.DialogueIndex`)))
  ;[1 1 1] Begin Dialogue
  (`/Engine/EditorBlueprintResources/StandardMacros.IncrementInt` (`self.DialogueIndex`)
    (:`  `
      ;[1 1 1] Check for Repetition
      (if _returnvalue
        (return "NewEnumerator0" _value)
        (else
          ;[1 1 1] Update Dialogue
          (`/Game/Game/Widgets/WBP_Dialogue.UpdateDialogueText` (`self.DialogueWidget`) (`self.DialogueIndex`) Speaker Dialogue OptionsText)
          ;[1 1 1] Play Dialogue Audio and Animation
          (`self.PlayDialogueAudio` (`local.DialogueAudio`))
          (`self.PlayAnimation` Animation)
          (return "NewEnumerator1" 0))))))

(fn `ClearDialogueProgress`
  ;[1 1 1] Clear Dialogue Progress
  (`BlueprintMapLibrary.Map_Clear` (`self.DialogueProgress`)))

(fn `CloseDialogue`
  ;[1 1 1] Close Dialogue Box
  (`Widget.RemoveFromParent` (`self.DialogueWidget`))
  ;[1 1 1] Stop Audio and Animation
  (bind _audiocomponent (`self.AudioComponent`)
    (:`then`
      (`AudioComponent.Stop` _audiocomponent)
      (bind _ascharacter (cast `Character` (`self.GetOwner`)))
      (`Character.StopAnimMontage` _ascharacter null)
      ;[1 1 1] Restore Movement
      (message `/Game/Game/Blueprints/Interactable/BPI_Interact.ConversationClosed` (`self.GetOwner`) ""))
    (:`else`)))

(fn `Dialogue`)

(fn `OpenDialogue`
  ;[1 1 1] Check for Widget
  (`/Engine/EditorBlueprintResources/StandardMacros.IsValid` (`self.DialogueWidget`)
    (:`Is Valid`
      _)
    (:`Is Not Valid`
      ;[1 1 1] Open Dialogue Box
      (bind _returnvalue (`|CreateWidget` "/Game/Game/Widgets/WBP_Dialogue.WBP_Dialogue_C" null self))
      (bind _output_get (set `self.DialogueWidget` _returnvalue))))
  (`UserWidget.AddToViewport` _output_get 0)
  ;[1 1 1] Advance Dialogue
  (`self.ProgressDialogue`))

(fn `PlayDialogueAudio`
  (params (Audio :type "SoundBase Soft Object Reference (by ref)"))
  (bind _audio (`local.Audio`))
  (bind _output (`|ConvertAsset` _audio))
  ;[1 1 1] Is Valid?
  (if (and (`KismetSystemLibrary.IsValidSoftObjectReference` Audio) (`self.bUseAudio?`))
    (`/Engine/EditorBlueprintResources/StandardMacros.IsValid` _output
      (:`Is Valid`
        ;[1 1 1] Set Sound
        (`AudioComponent.SetSound` (`self.AudioComponent`) _output)
        (`AudioComponent.Play` (`self.AudioComponent`) 0.0))
      (:`Is Not Valid`
        ;[1 1 1] Load Invalid Asset and Set Sound
        (`self.LoadDialogueAudio` _audio)))))

(fn `ProgressDialogue`
  ;[1 1 1] Reset Dialogue Index and Call Dialogue
  (set `self.DialogueIndex` -1)
  (`self.Dialogue`))

(fn `RemoveDialogueProgress`
  (params (ProgressSteps :type Integer))
  ;[1 1 1] Go to Previous Dialogue
  (for _index (range (+ ProgressSteps 1))
    (`BlueprintMapLibrary.Map_Remove` (`self.DialogueProgress`) (- (`self.DialogueIndex`) _index))))

(fn `SetDialogueBranch`
  (params (`Dialogue Branch` :type Name) (ProgressHandler :type "/Game/Game/Blueprints/Dialogue/EDialogueProgressStoreType Enum" :default "NewEnumerator0"))
  (switch `/Game/Game/Blueprints/Dialogue/EDialogueProgressStoreType` ProgressHandler
    (:`NewEnumerator1`
      ;[1 1 1] Add Dialogue Progress to Map
      (`BlueprintMapLibrary.Map_Add` (`self.BranchProgress`) (`self.ActiveDialogueBranch`) (make `/Game/Game/Blueprints/Dialogue/Struct_DialogueProgress` (`self.DialogueProgress`))))
    (:`NewEnumerator2`
      ;[1 1 1] Clear
      (`BlueprintMapLibrary.Map_Add` (`self.BranchProgress`) (`self.ActiveDialogueBranch`))))
  ;[1 1 1] Store Current Progress
  (set `self.DialogueProgress` (break `/Game/Game/Blueprints/Dialogue/Struct_DialogueProgress` (`BlueprintMapLibrary.Map_Find` (`self.BranchProgress`) (`local.Dialogue Branch`))))
  (set `self.ActiveDialogueBranch` (`local.Dialogue Branch`)))

(fn `UpdateSelectedOption`
  (params (ProgressIndex :type "Integer (by ref)") (OptionsIndex :type "Integer (by ref)"))
  ;[1 1 1] Set Dialogue for Selected Option
  (`BlueprintMapLibrary.Map_Add` (`self.DialogueProgress`) ProgressIndex OptionsIndex)
  (`self.ProgressDialogue`))