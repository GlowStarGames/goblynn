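; Dialogue component for Uncle Lazward, the dragon NPC who sends Lynn to collect Magic Nodes and bring down the undead's wards.
; Overrides Dialogue, switching on the active branch: Default quest briefing, Cont. short reminder, or Victory end-of-game talk.
; Chained AddDialogue calls play audio and montages; reply options converge on the same next line, and both long chains finish by switching to Cont.
; An alternate node line and random chatter remain unused.
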(fn `Dialogue`
  (bind _speaker (`self.Speaker`))
  (bind _speaker_2 (`self.Speaker`))
  ;[1 1 1] Begin Dialogue
  (`parent.Dialogue`)
  (set `self.Speaker` "Lazward the Wizardly")
  (switch `name` (`self.ActiveDialogueBranch`)
    (:`Default`
      ;[0 0 0] Default
      ;;[1 1 1] Greetings
      (bind (_state _optionsindex) (`self.AddDialogue` _speaker "Why, it's Lynn! Well aren't you a sight for sore eyes." (`|MakeArray` "> Hi, Uncle Lazward!" "> Uncle Lazward? That you, old man?" "> Uncle Lazward?! You startled me!" :!type "Text")))
      (switch `/Game/Game/Blueprints/Dialogue/Enum_DialogueState` _state
        (:`NewEnumerator0`
          (switch `int` _optionsindex
            (:`0`
              _)
            (:`1`
              _)
            (:`2`
              _))
          ;;[1 1 1] Welcome back
          (bind (_state_2 _optionsindex_2) (`self.AddDialogue` _speaker "Good to see you home. Your mother will be pleased. I only wish it were under better circumstances." (`|MakeArray` "> Why are you outside the city?" "> Are you... camping?" "> Shouldn't you be at home this time of night?" :!type "Text") "/Game/Old_Man_WAV/Misc_1.Misc_1" "/Game/Game/Blueprints/Animations/Montages/Montage_Dragon_Idle.Montage_Dragon_Idle"))
          (switch `/Game/Game/Blueprints/Dialogue/Enum_DialogueState` _state_2
            (:`NewEnumerator0`
              (switch `int` _optionsindex_2
                (:`0`
                  _)
                (:`1`
                  _)
                (:`2`
                  _))
              ;;[1 1 1] Undead invasion
              (bind (_state_3 _optionsindex_3) (`self.AddDialogue` (`self.Speaker`) "I've been chased out, my girl. The undead have invaded." (`|MakeArray` "> The undead? Wait, you mean the Lich Emporor's army?" "> ...Oh." "> Already? I thought we had more time before they'd reach us!" :!type "Text") "/Game/Old_Man_WAV/Misc_3_Cue.Misc_3_Cue" "/Game/Game/Blueprints/Animations/Montages/Montage_Dragon_Idle.Montage_Dragon_Idle"))
              (switch `/Game/Game/Blueprints/Dialogue/Enum_DialogueState` _state_3
                (:`NewEnumerator0`
                  (switch `int` _optionsindex_3
                    (:`0`
                      _)
                    (:`1`
                      _)
                    (:`2`
                      _))
                  ;;[1 1 1] Trapped inside
                  (bind (_state_4 _optionsindex_4) (`self.AddDialogue` (`self.Speaker`) "Oh, yes. And they've got wards up, keeping everybody in. Ghouls patrol the streets. I imagine everyone is holed up in their homes, as best they can be." (`|MakeArray` "> Is there anything we can do?" "> ...You got overpowered by ghouls?" "> What are we waiting for? We gotta go!" :!type "Text") "/Game/Old_Man_WAV/Misc_2_Cue.Misc_2_Cue" "/Game/Game/Blueprints/Animations/Montages/Montage_Dragon_Idle.Montage_Dragon_Idle"))
                  (switch `/Game/Game/Blueprints/Dialogue/Enum_DialogueState` _state_4
                    (:`NewEnumerator0`
                      (switch `int` _optionsindex_4
                        (:`0`
                          _)
                        (:`1`
                          _)
                        (:`2`
                          _))
                      ;;[1 1 1] Locked out
                      (bind (_state_5 _optionsindex_5) (`self.AddDialogue` (`self.Speaker`) "They've got a ward that keeps me out, or you know damn well I'd chase the lot out!" (`|MakeArray` "> What about me? What can I do?" "> Then I'll act without you. What are my options?" "> Then it's up to me! There must be something I can do." :!type "Text") "/Game/Old_Man_WAV/Grunt_2_Cue.Grunt_2_Cue" "/Game/Game/Blueprints/Animations/Montages/Montage_Dragon_Rawr.Montage_Dragon_Rawr"))
                      (switch `/Game/Game/Blueprints/Dialogue/Enum_DialogueState` _state_5
                        (:`NewEnumerator0`
                          (switch `int` _optionsindex_5
                            (:`0`
                              _)
                            (:`1`
                              _)
                            (:`2`
                              _))
                          ;;[1 1 1] You can get in
                          (bind (_state_6 _optionsindex_6) (`self.AddDialogue` (`self.Speaker`) "You? Yes, you might be able to get in. You're small. You won't be able to come back out though. Not once you're in. You'll be trapped, along with the rest of the villagers." (`|MakeArray` "> Can I do anything from the inside?" "> What good does that do us?" "> Can I still help if I'm trapped?" :!type "Text") "/Game/Old_Man_WAV/Misc_1_Cue.Misc_1_Cue" "/Game/Game/Blueprints/Animations/Montages/Montage_Dragon_Idle.Montage_Dragon_Idle"))
                          (switch `/Game/Game/Blueprints/Dialogue/Enum_DialogueState` _state_6
                            (:`NewEnumerator0`
                              (switch `int` _optionsindex_6
                                (:`0`
                                  _)
                                (:`1`
                                  _)
                                (:`2`
                                  _))
                              ;;[1 1 1] Objective: Destroy ward
                              (bind (_state_7 _optionsindex_7) (`self.AddDialogue` (`self.Speaker`) "Why, Lynn! You're going to bring down the wards." (`|MakeArray` "> How??" "> You want me to what now" "> I can do that??" :!type "Text") "/Game/Old_Man_WAV/Grunt_2_Cue.Grunt_2_Cue" "/Game/Game/Blueprints/Animations/Montages/Montage_Dragon_Rawr.Montage_Dragon_Rawr"))
                              (switch `/Game/Game/Blueprints/Dialogue/Enum_DialogueState` _state_7
                                (:`NewEnumerator0`
                                  (switch `int` _optionsindex_7
                                    (:`0`
                                      _)
                                    (:`1`
                                      _)
                                    (:`2`
                                      _))
                                  ;;[1 1 1] Collect Magic Nodes
                                  (bind (_state_8 _optionsindex_8) (`self.AddDialogue` (`self.Speaker`) "Look for the Magic Nodes scattered around the city. Their magic powers the wards. " (`|MakeArray` "> Go on..." "> Okay." "> Magic nodes. Got it!" :!type "Text") "/Game/Old_Man_WAV/Misc_3_Cue.Misc_3_Cue" "/Game/Game/Blueprints/Animations/Montages/Montage_Dragon_Idle.Montage_Dragon_Idle"))
                                  (switch `/Game/Game/Blueprints/Dialogue/Enum_DialogueState` _state_8
                                    (:`NewEnumerator0`
                                      (switch `int` _optionsindex_8
                                        (:`0`
                                          _)
                                        (:`1`
                                          _)
                                        (:`2`
                                          _))
                                      ;;[1 1 1] Spiky purple things
                                      (bind (_state_9 _optionsindex_9) (`self.AddDialogue` (`self.Speaker`) "Purple bottles, sparkling with Dark Magic. Dark Magic is also purple." (`|MakeArray` "> How many do I need?" "> And that'll bring down the wards?" "> Sparkling purple bottles. Got it!" :!type "Text") "/Game/Old_Man_WAV/Meh_Cue.Meh_Cue" "/Game/Game/Blueprints/Animations/Montages/Montage_Dragon_Idle.Montage_Dragon_Idle"))
                                      (switch `/Game/Game/Blueprints/Dialogue/Enum_DialogueState` _state_9
                                        (:`NewEnumerator0`
                                          (switch `int` _optionsindex_9
                                            (:`0`
                                              _)
                                            (:`1`
                                              _)
                                            (:`2`
                                              _))
                                          ;;[1 1 1] Three nodes
                                          (bind (_state_10 _optionsindex_10) (`self.AddDialogue` (`self.Speaker`) "You need to collect five Magic Nodes to bring down the wards." (`|MakeArray` "> Alright. I'm going in!" "> Let's get this over with." "> Leave it to me, Uncle Lazward!" :!type "Text") "/Game/Old_Man_WAV/Misc_1_Cue.Misc_1_Cue" "/Game/Game/Blueprints/Animations/Montages/Montage_Dragon_Idle.Montage_Dragon_Idle"))
                                          (switch `/Game/Game/Blueprints/Dialogue/Enum_DialogueState` _state_10
                                            (:`NewEnumerator0`
                                              (switch `int` _optionsindex_10
                                                (:`0`
                                                  _)
                                                (:`1`
                                                  _)
                                                (:`2`
                                                  _))
                                              ;;[1 1 1] Speak to me after
                                              (bind (_state_11 _optionsindex_11) (`self.AddDialogue` (`self.Speaker`) "Speak to me after you've brought down the wards. You can find me outside either gate to the village. I'll be watching your progress from overhead." (`|MakeArray` "> See you soon, Uncle Lazward!" "> Understood." "> I won't let you down!" :!type "Text") "/Game/Old_Man_WAV/Misc_1_Cue.Misc_1_Cue" "/Game/Game/Blueprints/Animations/Montages/Montage_Dragon_Idle.Montage_Dragon_Idle"))
                                              (switch `/Game/Game/Blueprints/Dialogue/Enum_DialogueState` _state_11
                                                (:`NewEnumerator0`
                                                  (switch `int` _optionsindex_11
                                                    (:`0`
                                                      _)
                                                    (:`1`
                                                      _)
                                                    (:`2`
                                                      _))
                                                  ;;[1 1 1] Bye
                                                  (bind (_state_12 _optionsindex_12) (`self.AddDialogue` (`self.Speaker`) "Good luck, my girl." (`|MakeArray` "> Thanks. I'll need it." "> I don't need it. I'm gonna kick some undead ass." "> You too! I love you!" :!type "Text") "/Game/Old_Man_WAV/Misc_1_Cue.Misc_1_Cue" "/Game/Game/Blueprints/Animations/Montages/Montage_Dragon_Idle.Montage_Dragon_Idle"))
                                                  (switch `/Game/Game/Blueprints/Dialogue/Enum_DialogueState` _state_12
                                                    (:`NewEnumerator0`
                                                      (switch `int` _optionsindex_12
                                                        (:`0`
                                                          _)
                                                        (:`1`
                                                          _)
                                                        (:`2`
                                                          _))
                                                      ;;[1 1 1] Set to Next Conversation
                                                      (`self.SetDialogueBranch` "Cont." "NewEnumerator1")
                                                      ;;[1 1 1] Close Dialogue
                                                      (`self.ClearDialogueProgress`)
                                                      (`self.CloseDialogue`))))))))))))))))))))))))))
    (:`Cont.`
      ;[0 0 0] Cont.
      ;;[1 1 1] Comment
      (bind _state_13 (`self.AddDialogue` (`self.Speaker`) "If you feel poorly, you should visit your mother. She's been making stew. It will perk you right up!" (`|MakeArray` "Bye, Uncle Lazward" :!type "Text")))
      (switch `/Game/Game/Blueprints/Dialogue/Enum_DialogueState` _state_13
        (:`NewEnumerator0`
          ;;[1 1 1] Close Dialogue
          (`self.ClearDialogueProgress`)
          (`self.CloseDialogue`))))
    (:`Victory`
      ;[0 0 0] Victory
      ;;[1 1 1] You did it!
      (bind (_state_14 _optionsindex_13) (`self.AddDialogue` _speaker_2 "Lynn! By dragonfire, you really did it!" (`|MakeArray` "> I made it out. Can you get in now?" "> It's done." "> Alright, Uncle Lazward! It's all yours!" :!type "Text")))
      (switch `/Game/Game/Blueprints/Dialogue/Enum_DialogueState` _state_14
        (:`NewEnumerator0`
          (switch `int` _optionsindex_13
            (:`0`
              _)
            (:`1`
              _)
            (:`2`
              _))
          ;;[1 1 1] The city is safe
          (bind (_state_15 _optionsindex_14) (`self.AddDialogue` _speaker_2 "I can get in! Oho! We'll have these undead cleared right out." (`|MakeArray` "> What comes next?" "> What now, old man?" "> What else can I do, Uncle Lazward?" :!type "Text") "/Game/Old_Man_WAV/Misc_1.Misc_1" "/Game/Game/Blueprints/Animations/Montages/Montage_Dragon_Idle.Montage_Dragon_Idle"))
          (switch `/Game/Game/Blueprints/Dialogue/Enum_DialogueState` _state_15
            (:`NewEnumerator0`
              (switch `int` _optionsindex_14
                (:`0`
                  _)
                (:`1`
                  _)
                (:`2`
                  _))
              ;;[1 1 1] Tutorial end
              (bind (_state_16 _optionsindex_15) (`self.AddDialogue` (`self.Speaker`) "My dear girl, you've reached the end of the content!" (`|MakeArray` "> The end of the content?" "> What" "> Please explain?" :!type "Text") "/Game/Old_Man_WAV/Misc_3_Cue.Misc_3_Cue" "/Game/Game/Blueprints/Animations/Montages/Montage_Dragon_Idle.Montage_Dragon_Idle"))
              (switch `/Game/Game/Blueprints/Dialogue/Enum_DialogueState` _state_16
                (:`NewEnumerator0`
                  (switch `int` _optionsindex_15
                    (:`0`
                      _)
                    (:`1`
                      _)
                    (:`2`
                      _))
                  ;;[1 1 1] Winner
                  (bind (_state_17 _optionsindex_16) (`self.AddDialogue` (`self.Speaker`) "The content! The game that the dev built. You've done it all!" (`|MakeArray` "> So this is the end of the game?" "> Pretty meta, old man." "> So... I won??" :!type "Text") "/Game/Old_Man_WAV/Misc_1_Cue.Misc_1_Cue" "/Game/Game/Blueprints/Animations/Montages/Montage_Dragon_Idle.Montage_Dragon_Idle"))
                  (switch `/Game/Game/Blueprints/Dialogue/Enum_DialogueState` _state_17
                    (:`NewEnumerator0`
                      (switch `int` _optionsindex_16
                        (:`0`
                          _)
                        (:`1`
                          _)
                        (:`2`
                          _))
                      ;;[1 1 1] Future quests
                      (bind (_state_18 _optionsindex_17) (`self.AddDialogue` (`self.Speaker`) "This is the end! You won! Perhaps in the future there will be more challenges for you. Add some quests. A boss fight. Who knows?" (`|MakeArray` "> That could be interesting." "> Did you say boss fights?" "> Fun!! I'm so excited!" :!type "Text") "/Game/Old_Man_WAV/Misc_2_Cue.Misc_2_Cue" "/Game/Game/Blueprints/Animations/Montages/Montage_Dragon_Idle.Montage_Dragon_Idle"))
                      (switch `/Game/Game/Blueprints/Dialogue/Enum_DialogueState` _state_18
                        (:`NewEnumerator0`
                          (switch `int` _optionsindex_17
                            (:`0`
                              _)
                            (:`1`
                              _)
                            (:`2`
                              _))
                          ;;[1 1 1] Anyway
                          (bind (_state_19 _optionsindex_18) (`self.AddDialogue` (`self.Speaker`) "Indeed. Run along now, Lynn, and see to the safety of the others. I'm going to go fight off the undead!" (`|MakeArray` "> Love you, Uncle Lazward!" "> Smell ya later, Uncle Lazward!" "> Bye, Uncle Lazward! I'm gonna go find my mom!" :!type "Text") "/Game/Old_Man_WAV/Grunt_2_Cue.Grunt_2_Cue" "/Game/FourEvilDragonsHP/Animations/DragonTheTerrorBringer/FlyAttackAnim_Montage.FlyAttackAnim_Montage"))
                          (switch `/Game/Game/Blueprints/Dialogue/Enum_DialogueState` _state_19
                            (:`NewEnumerator0`
                              (switch `int` _optionsindex_18
                                (:`0`
                                  _)
                                (:`1`
                                  _)
                                (:`2`
                                  _))
                              ;;[1 1 1] Set to Next Conversation
                              (`self.SetDialogueBranch` "Cont." "NewEnumerator1")
                              ;;[1 1 1] Close Dialogue
                              (`self.ClearDialogueProgress`)
                              (`self.CloseDialogue`))))))))))))))))