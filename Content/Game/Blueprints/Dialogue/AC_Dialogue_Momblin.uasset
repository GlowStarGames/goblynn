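; Dialogue component for Momblin, the player's goblin mother, who fusses over Lynn and offers stew as the quest progresses.
; The Dialogue override switches on the active branch: Assign Quest (also the default), Quest Incomplete and Quest Complete, the last pointing to Uncle Lazward.
; Each branch chains AddDialogue lines with reply options, voice cues and montages; replies converge on the same next line.
; The first two branches set QuestIncomplete before closing; completion just closes.
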(fn `Dialogue`
  (bind _speaker (`self.Speaker`))
  (bind _speaker_2 (`self.Speaker`))
  (bind _speaker_3 (`self.Speaker`))
  ;[1 1 1] Begin Dialogue
  (`parent.Dialogue`)
  (set `self.Speaker` "Momblin")
  (switch `name` (`self.ActiveDialogueBranch`)
    (:`Default`
      ;[0 0 0] Assign Quest
      ;;[1 1 1] My baby
      (bind (_state _optionsindex) (`self.AddDialogue` _speaker "Lynn! My sweet baby!" (`|MakeArray` "> Hi, Mama!" "> Calm down; I'm okay." "> Mommy, I'm hungry!" :!type "Text") :!label _label))
      (switch `/Game/Game/Blueprints/Dialogue/Enum_DialogueState` _state
        (:`NewEnumerator0`
          (switch `int` _optionsindex
            (:`0`
              _)
            (:`1`
              _)
            (:`2`
              _))
          ;;[1 1 1] Proud of you
          (bind (_state_2 _optionsindex_2) (`self.AddDialogue` _speaker "Are you okay? Are you being careful? Are you injured?" (`|MakeArray` "> I'm being careful! But I have to do this." "> I'm fine, Mama. Stop fussing!" "> Mama, can I have some stew?" :!type "Text") "/Game/HumanVocalizations/HumanFemaleC/Cues/voice_female_c_battle_shout_02_Cue.voice_female_c_battle_shout_02_Cue" "/Game/UndeadPack/EnemyGoblin/Animations/Anim_Arg_Montage.Anim_Arg_Montage"))
          (switch `/Game/Game/Blueprints/Dialogue/Enum_DialogueState` _state_2
            (:`NewEnumerator0`
              (switch `int` _optionsindex_2
                (:`0`
                  _)
                (:`1`
                  _)
                (:`2`
                  _))
              ;;[1 1 1] Stew
              (bind (_state_3 _optionsindex_3) (`self.AddDialogue` (`self.Speaker`) "I'm so proud of you, baby. Eat some stew and be strong, okay?" (`|MakeArray` "> Thank you, Mama!" "> Mooom, I'm fine!" "> Yaaay! Yummy!" :!type "Text") "/Game/HumanVocalizations/HumanFemaleC/Cues/voice_female_c_effort_push_01_Cue.voice_female_c_effort_push_01_Cue" "/Game/Game/Blueprints/Animations/Montages/Montage_Goblin_Hit.Montage_Goblin_Hit"))
              (switch `/Game/Game/Blueprints/Dialogue/Enum_DialogueState` _state_3
                (:`NewEnumerator0`
                  (switch `int` _optionsindex_3
                    (:`0`
                      _)
                    (:`1`
                      _)
                    (:`2`
                      _))
                  ;;[1 1 1] Set to Next Conversation
                  (`self.SetDialogueBranch` "QuestIncomplete" "NewEnumerator1")
                  ;;[1 1 1] Close Dialogue
                  (`self.ClearDialogueProgress`)
                  (`self.CloseDialogue`))))))))
    (:`AssignQuest`
      (goto _label))
    (:`QuestIncomplete`
      ;[0 0 0] QuestIncomplete
      ;;[1 1 1] Check-In
      (bind (_state_4 _optionsindex_4) (`self.AddDialogue` _speaker_2 "Hey, sweetie. How is your quest?" (`|MakeArray` "> Hi, Mama! It's good." "> I can handle it." "> It's hard!" :!type "Text")))
      (switch `/Game/Game/Blueprints/Dialogue/Enum_DialogueState` _state_4
        (:`NewEnumerator0`
          (switch `int` _optionsindex_4
            (:`0`
              _)
            (:`1`
              _)
            (:`2`
              _))
          ;;[1 1 1] Proud of you
          (bind (_state_5 _optionsindex_5) (`self.AddDialogue` _speaker_2 "My poor baby works so hard. Have some stew!" (`|MakeArray` "> Thank you, Mama!" :!type "Text") "/Game/HumanVocalizations/HumanFemaleC/Cues/voice_female_c_effort_push_01_Cue.voice_female_c_effort_push_01_Cue" "/Game/Game/Blueprints/Animations/Montages/Montage_Goblin_Hit.Montage_Goblin_Hit"))
          (switch `/Game/Game/Blueprints/Dialogue/Enum_DialogueState` _state_5
            (:`NewEnumerator0`
              (switch `int` _optionsindex_5
                (:`0`
                  ;;[1 1 1] Set to Next Conversation
                  (`self.SetDialogueBranch` "QuestIncomplete" "NewEnumerator1")
                  ;;[1 1 1] Close Dialogue
                  (`self.ClearDialogueProgress`)
                  (`self.CloseDialogue`))))))))
    (:`QuestComplete`
      ;[0 0 0] QuestComplete
      ;;[1 1 1] You did it!
      (bind (_state_6 _optionsindex_6) (`self.AddDialogue` _speaker_3 "You did it! You brought down the wards!" (`|MakeArray` "> We can get out now!" "> The undead will be gone soon." "> I did it!" :!type "Text")))
      (switch `/Game/Game/Blueprints/Dialogue/Enum_DialogueState` _state_6
        (:`NewEnumerator0`
          (switch `int` _optionsindex_6
            (:`0`
              _)
            (:`1`
              _)
            (:`2`
              _))
          ;;[1 1 1] Talk to Lazward
          (bind (_state_7 _optionsindex_7) (`self.AddDialogue` _speaker_3 "I'm so proud of you sweetie. Have you talked to Uncle Lazward yet?" (`|MakeArray` "> Not yet." "> I want to keep looking around first!" "> I'm going right now!" :!type "Text") "/Game/HumanVocalizations/HumanFemaleC/Cues/voice_female_c_effort_push_01_Cue.voice_female_c_effort_push_01_Cue" "/Game/Game/Blueprints/Animations/Montages/Montage_Goblin_Hit.Montage_Goblin_Hit"))
          (switch `/Game/Game/Blueprints/Dialogue/Enum_DialogueState` _state_7
            (:`NewEnumerator0`
              (switch `int` _optionsindex_7
                (:`0`
                  _)
                (:`1`
                  _)
                (:`2`
                  _))
              ;;[1 1 1] Talk to Lazward
              (bind (_state_8 _optionsindex_8) (`self.AddDialogue` _speaker_3 "He's outside the village when you're ready. Have some stew, honey." (`|MakeArray` "> Thank you, Mama!" :!type "Text") "/Game/HumanVocalizations/HumanFemaleC/Cues/voice_female_c_effort_push_01_Cue.voice_female_c_effort_push_01_Cue" "/Game/Game/Blueprints/Animations/Montages/Montage_Goblin_Hit.Montage_Goblin_Hit"))
              (switch `/Game/Game/Blueprints/Dialogue/Enum_DialogueState` _state_8
                (:`NewEnumerator0`
                  (switch `int` _optionsindex_8
                    (:`0`
                      ;;[1 1 1] Close Dialogue
                      (`self.ClearDialogueProgress`)
                      (`self.CloseDialogue`))))))))))))