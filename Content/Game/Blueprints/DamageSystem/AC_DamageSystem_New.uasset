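; Actor component that manages an actor's health, damage intake, healing and death state.
; TakeDamage routes a damage info struct through the CanBeDamaged macro, which uses dead, invincible and blocking states to choose block, damage or no damage.
; Dispatchers broadcast blocks with parry eligibility, deaths, and damage responses when the owner is interruptible or interruption is forced.
; Heal restores health up to the maximum, only while alive.
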(fn `Heal`
  (params (HealAmount :type "Float (double-precision)"))
  (returns (NewHealth :type "Float (double-precision)"))
  ;[1 1 1] The Dead Cannot Heal
  (if (not (`self.bIsDead`))
    (bind _output_get (set `self.Health` (`KismetMathLibrary.FClamp` (+ HealAmount (`self.Health`)) 0.0 (`self.MaxHealth`))))
    (return _output_get)))

(fn `TakeDamage`
  (params (DamageInfo :type "/Game/Game/Blueprints/DamageSystem/S_DamageInfo Structure"))
  (returns (bWasDamaged :type Boolean))
  (bind (_damageamount _damagetype _damageresponse _bshoulddamageinvincible _bcanbeblocked _bcanbeparried _bshouldforceinterrupt) (break `/Game/Game/Blueprints/DamageSystem/S_DamageInfo` DamageInfo))
  ;[1 1 1] Can Be Damaged?
  (`self.CanBeDamaged` _bshoulddamageinvincible _bcanbeblocked
    (:`BlockDamage`
      ;[1 1 1] No Damage
      (`self.OnBlocked` _bcanbeparried))
    (:`DoDamage`
      ;[1 1 1] Set Damage and Check Death
      (bind _output_get (set `self.Health` (- (`self.Health`) _damageamount)))
      (if (<= _output_get 0.0)
        ;[1 1 1] Die
        (bind _output_get_2 (set `self.bIsDead` true))
        (`self.OnDeath`)
        (else
          ;[1 1 1] Response to Damage
          (if (or (`self.bIsInterruptible`) _bshouldforceinterrupt)
            (`self.OnDamageResponse` _damageresponse)
            (`KismetSystemLibrary.PrintString` "Damage Called")
            (else
              (`KismetSystemLibrary.PrintString` "Damage Interrupted")
              (return false)))))
      (return _output_get_2))
    (:`NoDamage`
      _))
  (`KismetSystemLibrary.PrintString` "No Damage")
  (return false))